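; Player equipment component that tracks an item and optional equipment actor per slot type, using the inventory component and a player interface.
; Equipping reads data table rows, sets skeletal meshes that follow the master pose or attach to a bone, and swaps with occupied slots.
; Unequipping returns items to inventory or drops them, updating slot widgets.
; Saving stores item IDs and actor classes; loading respawns actors and re-equips.
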(event Custom|Initialize
  (bind _playerinventory (CallFunction|GetPlayerInventory))
  (CallFunction|SetupEquipment)
  (if (Utilities|DoesObjectImplementInterface (Components|GetOwner) "/Game/OpenRPG/EquipmentSystem/Blueprints/BPI_Equipment.BPI_Equipment_C")
    (Utilities|IsValid _playerinventory
      (:Is%20Valid
        (Variables|Default|SetPlayerInventoryReference _playerinventory)
        (Default|Initialize (Variables|Default|GetEquipmentSlotsContainerWidget) self)
        (CallFunction|LoadEquipment)
        (Development|PrintString "Your BPC_Equipment is configured successfully!!!" true true "(R=1.000000,G=0.086574,B=0.000000,A=1.000000)" 1e+01))
      (:Is%20Not%20Valid
        (Development|PrintString "Error: Your player doesnt have the PlayerInventory component" true true "(R=1.000000,G=0.086574,B=0.000000,A=1.000000)" 1e+01)))
    (else
      (Development|PrintString "Error: Your player doesnt implement the required BPI_Equipment interface" true true "(R=1.000000,G=0.086574,B=0.000000,A=1.000000)" 1e+01))))

(event Custom|UpdateEquipmentSlot
  (params (Slot :type e_EquipmentType%20Enum :default "NewEnumerator0"))
  (Default|Update (CallFunction|GetEquipmentSlotWidget Slot)))

(fn GetEquipmentDatafromRow
  (params (RowName :type Name))
  (bind _returnvalue (Utilities|GetDataTableRow "/Game/OpenRPG/EquipmentSystem/Datatables/DT_Equipment.DT_Equipment" RowName)
    (:then
      (return _returnvalue))
    (:RowNotFound
      (return ""))))

(fn GetEquipmentSlotWidget
  (params (SlotType :type e_EquipmentType%20Enum :default "NewEnumerator0"))
  (LocalVariables|SetLocalType SlotType)
  (bind _array_element (Utilities|Array|ForEachLoopwithBreak (Variables|/Game/OpenRPG/EquipmentSystem/Widgets/WB_EquipmentSlotsContainer.WB_EquipmentSlotsContainer_C|GetSlots (Variables|Default|GetEquipmentSlotsContainerWidget)) :!label _label)
    (:LoopBody
      (if (Utilities|Enum|Equal(Enum) (Variables|/Game/OpenRPG/EquipmentSystem/Widgets/WB_EquipmentSlot.WB_EquipmentSlot_C|GetType _array_element) (LocalVariables|GetLocalType))
        (LocalVariables|SetLocalSlotWidget _array_element)
        (goto _label Break)))
    (:Completed
      (return (LocalVariables|GetLocalSlotWidget)))))

(fn GetIteminSlot
  (params (SlotType :type e_EquipmentType%20Enum :default "NewEnumerator0"))
  (return (.Value (Utilities|Map|Find (Variables|Default|GetEquipment) SlotType)) (.Value (Utilities|Map|Find (Variables|Default|GetEquipmentActors) SlotType))))

(fn EquipItem
  (params (Item :type Integer) (FromInventorySlot :type Integer) (EquipmentActor :type BP%20Base%20Equipment%20Object%20Reference))
  ;[0.08879 0.8399 1] This part of the code just extracts the necessary data and set it, giving warnings when something is not correctly set.
  (LocalVariables|SetLocalItemID Item)
  (LocalVariables|SetLocalClickedInventorySlot FromInventorySlot)
  (LocalVariables|SetLocalEquipmentActor EquipmentActor)
  (Utilities|IsValid (Variables|Default|GetPlayerInventoryReference)
    (:Is%20Valid
      (bind _mesh (Class|BPIEquipment|GetPlayerMesh(Message) (Components|GetOwner)))
      (bind _output_get (LocalVariables|SetLocalPlayerMesh _mesh))
      (Utilities|IsValid _output_get
        (:Is%20Valid
          (bind _output_get_2 (LocalVariables|SetLocalItemData (Default|GetItemDatafromID (Variables|Default|GetPlayerInventoryReference) (LocalVariables|GetLocalItemID))))
          (if (Utilities|Name|NotEqual(Name) (.EquipmentDataRowName (Utilities|Struct|Breaks_ItemData _output_get_2)) "None")
            (bind _output_get_3 (LocalVariables|SetLocalEquipmentData (CallFunction|GetEquipmentDatafromRow (.EquipmentDataRowName (Utilities|Struct|Breaks_ItemData _output_get_2)))))
            (LocalVariables|SetLocalSlotType (Utilities|Struct|Breaks_EquipmentData _output_get_3))
            (bind _meshcomponent (Class|BPIEquipment|GetEquipmentMeshComponentbyType(Message) (Components|GetOwner) (LocalVariables|GetLocalSlotType)))
            (bind _output_get_4 (LocalVariables|SetLocalMeshComponent _meshcomponent)) ; We get the mesh component of the player that we are going to update
            (Utilities|IsValid _output_get_4
              (:Is%20Valid
                (bind _output_get_5 (LocalVariables|SetLocalEquippedItemID (.ItemID (CallFunction|GetIteminSlot (LocalVariables|GetLocalSlotType))))) ; We extract the ID of the item that could be equipped when we want to equip in that slot
                (if (== _output_get_5 -1) ; Is the slot empty?
                  ;[1 0.91 0.07485] This part is responsible of the visual equipment, it updates the player pawn with the skeletal mesh of the item that we are going to equip
                  (Utilities|IsValid (Utilities|Struct|Breaks_EquipmentData (LocalVariables|GetLocalEquipmentData)) ; If the mesh isnt valid we skip the visual logic part
                    (:Is%20Valid
                      (Class|SkinnedMeshComponent|SetSkeletalMesh (LocalVariables|GetLocalMeshComponent) (Utilities|Struct|Breaks_EquipmentData (LocalVariables|GetLocalEquipmentData)) true) ; We set the mesh of that component to the one in the equipment data
                      (if (Utilities|Name|Equal(Name) (Utilities|Struct|Breaks_EquipmentData (LocalVariables|GetLocalEquipmentData)) "None") ; If we want to attach the component in a particular bone with custom transform this will have a valid value (only recommended for weapons)
                        (Class|SkinnedMeshComponent|SetMasterPoseComponent (LocalVariables|GetLocalMeshComponent) (LocalVariables|GetLocalPlayerMesh) false) ; If the skeletal mesh has the same skeleton as our player, this function will make it to fit it
                        (else
                          (Transformation|AttachComponentToComponent (LocalVariables|GetLocalMeshComponent) (LocalVariables|GetLocalPlayerMesh) (Utilities|Struct|Breaks_EquipmentData (LocalVariables|GetLocalEquipmentData)) "KeepRelative" "KeepRelative" "KeepRelative" true)
                          (Transformation|SetRelativeTransform (LocalVariables|GetLocalMeshComponent) (Utilities|Struct|Breaks_EquipmentData (LocalVariables|GetLocalEquipmentData)) false false))))
                    (:Is%20Not%20Valid
                      _))
                  (Utilities|Map|Add (Variables|Default|GetEquipment) (LocalVariables|GetLocalSlotType) (LocalVariables|GetLocalItemID))
                  (Utilities|Map|Add (Variables|Default|GetEquipmentActors) (LocalVariables|GetLocalSlotType) (LocalVariables|GetLocalEquipmentActor))
                  (Utilities|IsValid (LocalVariables|GetLocalEquipmentActor)
                    (:Is%20Valid
                      (Default|OnEquipped (LocalVariables|GetLocalEquipmentActor)))
                    (:Is%20Not%20Valid
                      _))
                  (CallFunction|UpdateEquipmentSlot (LocalVariables|GetLocalSlotType))
                  (if (== (LocalVariables|GetLocalClickedInventorySlot) -1) ; If false it means the equip comes from an inventory slot
                    _
                    (else
                      (Default|RemoveIndexAmount (Variables|Default|GetPlayerInventoryReference) (LocalVariables|GetLocalClickedInventorySlot) 1) ; So we remove the item in that slot, if not we would see it in the equipment slot and in the inventory
                    ))
                  (Default|CallOnItemEquipped (LocalVariables|GetLocalItemID) (LocalVariables|GetLocalSlotType))
                  (return)
                  (else
                    ;[1 0.09225 0.142] This part of the code makes a swap between the item that we know its already equipped and the one that we want to equip
                    (Default|RemoveIndexAmount (Variables|Default|GetPlayerInventoryReference) (LocalVariables|GetLocalClickedInventorySlot) 1) ; First we clean the slot of the item that we are going to equip (we have it stored in the LocalItemID variable)
                    (CallFunction|UnequipItem (LocalVariables|GetLocalSlotType) (LocalVariables|GetLocalClickedInventorySlot) false)
                    (CallFunction|EquipItem (LocalVariables|GetLocalItemID) -1 (LocalVariables|GetLocalEquipmentActor))
                    (return))))
              (:Is%20Not%20Valid
                (Development|PrintString "Error: The function GetEquipmentMeshComponentByType in your player isnt implemented correctly, its returning a not valid mesh component" true true "(R=0.000000,G=0.660000,B=1.000000,A=1.000000)" 2e+01)
                (return)))
            (else
              (Development|PrintString "Invalid row name to get the equipment data")
              (return))))
        (:Is%20Not%20Valid
          (Development|PrintString "Error: The function GetPlayerMesh in your player isnt implemented correctly, its returning a not valid mesh component")
          (return))))
    (:Is%20Not%20Valid
      (Development|PrintString "Error: The InventoryComponent reference in the EquipmentComponent is not valid!" true true "(R=0.000000,G=0.660000,B=1.000000,A=1.000000)" 8.0)
      (return))))

(fn UnequipItem
  (params (SlotType :type e_EquipmentType%20Enum :default "NewEnumerator0") (ToSpecificInventoryIndex :type Integer) (Drop? :type Boolean))
  (LocalVariables|SetLocalSlotType SlotType)
  (LocalVariables|SetLocalSpecificIndex ToSpecificInventoryIndex)
  (LocalVariables|SetLocalDrop Drop?)
  (Utilities|IsValid (Variables|Default|GetPlayerInventoryReference)
    (:Is%20Valid
      (bind _meshcomponent (Class|BPIEquipment|GetEquipmentMeshComponentbyType(Message) (Components|GetOwner) (LocalVariables|GetLocalSlotType)))
      (bind _output_get (LocalVariables|SetLocalMeshComponent _meshcomponent)) ; We get the mesh component of the player that we are going to update
      (Utilities|IsValid _output_get
        (:Is%20Valid
          (LocalVariables|SetLocalEquippedItemID (.ItemID (CallFunction|GetIteminSlot (LocalVariables|GetLocalSlotType)))) ; We get the current equipped item in the slot
          (LocalVariables|SetLocalEquipmentActor (.EquipmentActor (CallFunction|GetIteminSlot (LocalVariables|GetLocalSlotType))))
          (if (LocalVariables|GetLocalDrop)
            (Default|DropItem (Variables|Default|GetPlayerInventoryReference) (Utilities|Struct|Makes_InventoryItem (LocalVariables|GetLocalEquippedItemID) 1))
            (elif (!= (LocalVariables|GetLocalSpecificIndex) -1) ; If true it means we have to unequip to a specifil inventory index (we are dragging from the equipment slot to an inventory slot)
              (if (Default|IsSlotEmpty? (Variables|Default|GetPlayerInventoryReference) (LocalVariables|GetLocalSpecificIndex)) ; If the slot is empty it means we can drop the item in the inventory slot
                (Default|AddItemtoIndex (Variables|Default|GetPlayerInventoryReference) (Utilities|Struct|Makes_InventoryItem (LocalVariables|GetLocalEquippedItemID) 1) (LocalVariables|GetLocalSpecificIndex)) ; We add it
                (else
                  (Development|PrintString "Drop index has already an item")
                  (return false)))
              (else
                (bind _success_ (Default|AddIItem (Variables|Default|GetPlayerInventoryReference) (Utilities|Struct|Makes_InventoryItem (LocalVariables|GetLocalEquippedItemID) 1))) ; We unequip in the first emty slot
                (if _success_
                  _
                  (else
                    (Development|PrintString "Error while unequipping the item, maybe not enough space in inventory")
                    (return false))))))
          (Class|SkinnedMeshComponent|SetSkeletalMesh (LocalVariables|GetLocalMeshComponent) 0 true) ; Resets the visual equipment, it simulates that we unequipped the item
          (Utilities|Map|Add (Variables|Default|GetEquipment) (LocalVariables|GetLocalSlotType) -1)
          (Utilities|Map|Add (Variables|Default|GetEquipmentActors) (LocalVariables|GetLocalSlotType) 0)
          (Utilities|IsValid (LocalVariables|GetLocalEquipmentActor)
            (:Is%20Valid
              (Default|OnUnequipped (LocalVariables|GetLocalEquipmentActor)))
            (:Is%20Not%20Valid
              _))
          (CallFunction|UpdateEquipmentSlot (LocalVariables|GetLocalSlotType))
          (Default|CallOnItemUnequipped (LocalVariables|GetLocalEquippedItemID) (LocalVariables|GetLocalSlotType) (LocalVariables|GetLocalDrop))
          (return true))
        (:Is%20Not%20Valid
          (Development|PrintString "Error: The function GetEquipmentMeshComponentByType in your player isnt implemented correctly, its returning a not valid mesh component" true true "(R=0.000000,G=0.660000,B=1.000000,A=1.000000)" 2e+01)
          (return false))))
    (:Is%20Not%20Valid
      (Development|PrintString "Error: The InventoryComponent reference in the EquipmentComponent is not valid!")
      (return false))))

(fn ToggleEquipmentVisibility
  (LocalVariables|SetLocalParentWidget (Widget|GetParent (Variables|Default|GetEquipmentSlotsContainerWidget)))
  (while (Utilities|IsValid (LocalVariables|GetLocalParentWidget))
    (LocalVariables|SetLocalWidgetToToggle (LocalVariables|GetLocalParentWidget))
    (LocalVariables|SetLocalParentWidget (Widget|GetParent (LocalVariables|GetLocalParentWidget))))
  (Widget|SetVisibility (LocalVariables|GetLocalWidgetToToggle) (select (Widget|IsVisible (LocalVariables|GetLocalWidgetToToggle)) "Hidden" "Visible"))
  (return))

(fn SaveEquipment
  (Utilities|IsValid (Variables|Default|GetSaveEquipmentObject)
    (:Is%20Valid
      _)
    (:Is%20Not%20Valid
      (bind _returnvalue (SaveGame|CreateSaveGameObject "/Game/OpenRPG/EquipmentSystem/Blueprints/EquipmentSave.EquipmentSave_C"))
      (Variables|Default|SetSaveEquipmentObject _returnvalue)))
  (Variables|/Game/OpenRPG/EquipmentSystem/Blueprints/EquipmentSave.EquipmentSave_C|SetSavedEquipment (Variables|Default|GetSaveEquipmentObject) (Variables|Default|GetEquipment))
  (bind _keys (Utilities|Map|Keys (Variables|Default|GetEquipmentActors)))
  (for _array_element _keys
    (Utilities|Map|Add (Variables|/Game/OpenRPG/EquipmentSystem/Blueprints/EquipmentSave.EquipmentSave_C|GetSavedEquipmentActorClasses (Variables|Default|GetSaveEquipmentObject)) _array_element (Utilities|GetClass (.Value (Utilities|Map|Find (Variables|Default|GetEquipmentActors) _array_element)))))
  (SaveGame|SaveGametoSlot (Variables|Default|GetSaveEquipmentObject) (Variables|Default|GetSaveEquipmentSlotName))
  (Default|CallOnEquipmentSaved)
  (return))

(fn LoadEquipment
  (bind _returnvalue (SaveGame|DoesSaveGameExist (Variables|Default|GetSaveEquipmentSlotName)))
  (if _returnvalue
    (Utilities|IsValid (Variables|Default|GetSaveEquipmentObject)
      (:Is%20Valid
        _)
      (:Is%20Not%20Valid
        (bind _returnvalue_2 (SaveGame|LoadGamefromSlot (Variables|Default|GetSaveEquipmentSlotName)))
        (bind _asequipment_save (Utilities|Casting|CastToEquipmentSave _returnvalue_2)
          (:then
            (Variables|Default|SetSaveEquipmentObject _asequipment_save))
          (:CastFailed
            (return false)))))
    (bind _keys (Utilities|Map|Keys (Variables|/Game/OpenRPG/EquipmentSystem/Blueprints/EquipmentSave.EquipmentSave_C|GetSavedEquipment (Variables|Default|GetSaveEquipmentObject))))
    (for _array_element _keys
      (LocalVariables|SetLocalCurrentLoopEquipmentSlot _array_element)
      (bind _output_get (LocalVariables|SetLocalCurrentLoopEquipmentItemID (.Value (Utilities|Map|Find (Variables|/Game/OpenRPG/EquipmentSystem/Blueprints/EquipmentSave.EquipmentSave_C|GetSavedEquipment (Variables|Default|GetSaveEquipmentObject)) (LocalVariables|GetLocalCurrentLoopEquipmentSlot)))))
      (if (!= _output_get -1)
        (if (Utilities|IsValidClass (.Value (Utilities|Map|Find (Variables|/Game/OpenRPG/EquipmentSystem/Blueprints/EquipmentSave.EquipmentSave_C|GetSavedEquipmentActorClasses (Variables|Default|GetSaveEquipmentObject)) (LocalVariables|GetLocalCurrentLoopEquipmentSlot))))
          (bind _returnvalue_3 (Game|SpawnActorfromClass (.Value (Utilities|Map|Find (Variables|/Game/OpenRPG/EquipmentSystem/Blueprints/EquipmentSave.EquipmentSave_C|GetSavedEquipmentActorClasses (Variables|Default|GetSaveEquipmentObject)) (LocalVariables|GetLocalCurrentLoopEquipmentSlot))) (Math|Transform|MakeTransform "0, 0, 0" "0, 0, 0" "1,1,1") "Undefined" 0 (LocalVariables|GetLocalCurrentLoopEquipmentItemID) (Default|GetItemDatafromID (Variables|Default|GetPlayerInventoryReference) (LocalVariables|GetLocalCurrentLoopEquipmentItemID)) (Variables|Default|GetPlayerInventoryReference) 0)))
        (CallFunction|EquipItem (LocalVariables|GetLocalCurrentLoopEquipmentItemID) -1 _returnvalue_3)))
    (Default|CallOnEquipmentLoaded)
    (return true)
    (else
      (return false))))

(fn SetupEquipment
  (bind _enumvalue (|ForEache_EquipmentType)
    (:LoopBody
      (Utilities|Map|Add (Variables|Default|GetEquipment) _enumvalue -1))
    (:then
      (bind _foundwidgets (Widget|GetAllWidgetsOfClass "/Game/OpenRPG/EquipmentSystem/Widgets/WB_EquipmentSlotsContainer.WB_EquipmentSlotsContainer_C" false))
      (Utilities|IsValid (Utilities|Array|Get(acopy) _foundwidgets)
        (:Is%20Valid
          (Variables|Default|SetEquipmentSlotsContainerWidget (Utilities|Array|Get(acopy) _foundwidgets))
          (return))
        (:Is%20Not%20Valid
          (Development|PrintString "Unable to find the equipment slots container widget")
          (return))))))