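; BP_BaseEquipment is the base class for equippable items in the OpenRPG inventory system.
; Using the item calls the parent logic, then passes its ID, source slot and actor to the player's BPC_Equipment component and fires the equip and item-used events.
; An error prints if that component is missing.
; OnEquipped is an empty hook, while OnUnequipped destroys the actor.
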(event Custom|OnEquipped)

(event Custom|OnUnequipped
  (Actor|DestroyActor))

(event EventUseItem
  (params (Clicked%20Slot%20Index :type Integer))
  (bind _player (Variables|Default|GetPlayer))
  (bind _returnvalue (Actor|GetComponentbyClass _player "/Game/OpenRPG/EquipmentSystem/Blueprints/BPC_Equipment.BPC_Equipment_C"))
  ;[0.1043 1 0.1512] If you have your own way to equip items, it should be implemented here. This is my way of doing it
  (|CallParentFunction Clicked%20Slot%20Index)
  (Utilities|IsValid _returnvalue
    (:Is%20Valid
      (Default|EquipItem _returnvalue (Variables|Default|GetItemID) (Variables|Default|GetClickedSlotIndex) self)
      (CallFunction|OnEquipped)
      (CallFunction|OnItemUsed) ; Just if you want to use it :D
    )
    (:Is%20Not%20Valid
      (Development|PrintString "Error: You cant use equipment items because the BPI_Equipment interface doesnt return a valid equipment component"))))

(fn ConstructionScript
  (|CallParentFunction))