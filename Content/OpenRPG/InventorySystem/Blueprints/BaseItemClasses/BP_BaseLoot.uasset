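; BP_BaseLoot is the base class for usable loot items that open into a set of items in the player's inventory.
; On use, ManageLoot looks up the item's loot row in DT_Loot and tries to add those items to the inventory component.
; Success removes one item from the clicked slot and calls OnItemUsed, while failure prints a message.
; The actor destroys itself either way.
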(event EventUseItem
  (params (Clicked%20Slot%20Index :type Integer))
  (|CallParentFunction Clicked%20Slot%20Index)
  (bind _success_ (CallFunction|ManageLoot))
  (if _success_
    (CallFunction|OnItemUsed))
  (Actor|DestroyActor))

(fn ConstructionScript
  (|CallParentFunction))

(fn GetLootfromID
  (params (LootRowName :type Name))
  (bind _returnvalue (Utilities|GetDataTableRow "/Game/OpenRPG/InventorySystem/Datatables/DT_Loot.DT_Loot" LootRowName)
    (:then
      (return (Utilities|Struct|Breaks_Loot _returnvalue)))
    (:RowNotFound
      (return 0))))

(fn ManageLoot
  (bind _itemdata (Variables|Default|GetItemData))
  (bind _lootdatarowname (Utilities|Struct|Breaks_ItemData _itemdata))
  (if (Utilities|Name|NotEqual(Name) _lootdatarowname "None")
    (bind _output_get (LocalVariables|SetLocalLoot (CallFunction|GetLootfromID _lootdatarowname)))
    (bind _success_ (Default|AddItems (Variables|Default|GetPlayerInventoryComponent) _output_get))
    (if _success_
      (Default|RemoveIndexAmount (Variables|Default|GetPlayerInventoryComponent) (Variables|Default|GetClickedSlotIndex) 1)
      (return true)
      (else
        (Development|PrintString "Not enough space to open the loot!")
        (return false)))
    (else
      (Development|PrintString "Invalid loot row name")
      (return false))))