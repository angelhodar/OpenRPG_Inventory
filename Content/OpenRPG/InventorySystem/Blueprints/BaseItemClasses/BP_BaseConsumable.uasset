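; BP_BaseConsumable is the base class for consumable items in the inventory system.
; UseItem calls the parent, then runs OnItemUsed, where item-specific logic can clear UsedSuccessfully when the item cannot be used.
; On success it removes one unit from the clicked slot through PlayerInventoryComponent, and in either case it destroys the item actor afterwards.
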(event EventUseItem
  (params (Clicked%20Slot%20Index :type Integer))
  ;[0.1043 1 0.1512] I put this by default, modify it to your own preference.
  (|CallParentFunction Clicked%20Slot%20Index)
  (Utilities|FlowControl|Sequence
    (:then_0
      (CallFunction|OnItemUsed) ; First we execute the overriden item logic. If the item cant be used, make sure you set the UsedSuccessfully boolean to false (for example you try to use a health potion but the health is at 100%)
    )
    (:then_1
      (if (Variables|Default|GetUsedSuccessfully?)
        (Default|RemoveIndexAmount (Variables|Default|GetPlayerInventoryComponent) (Variables|Default|GetClickedSlotIndex) 1))
      (Actor|DestroyActor) ; Then we just destroy it
    )))

(fn ConstructionScript
  (|CallParentFunction))