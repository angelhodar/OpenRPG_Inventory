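; Demo storage actor for the inventory system, with a configurable mesh and interaction radius, that players open when nearby.
; Overlapping its sphere shows a "Storage" key prompt and registers the actor as NearbyStorage on the player's BPC_PlayerInventory.
; OnInteract lazily initializes the BPCStorage component, toggles its widget and refreshes the container view.
; Leaving the sphere clears the reference, hides the prompt, saves an initialized inventory and closes its open widget.
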(event OnComponentBeginOverlap(InteractColision)
  (params (OverlappedComponent :type Primitive%20Component%20Object%20Reference) (OtherActor :type Actor%20Object%20Reference) (OtherComp :type Primitive%20Component%20Object%20Reference) (OtherBodyIndex :type Integer) (bFromSweep :type Boolean) (SweepResult :type Hit%20Result%20Structure%20%28by%20ref%29))
  (bind _returnvalue (Actor|GetComponentbyClass OtherActor "/Game/OpenRPG/InventorySystem/Blueprints/Components/BPC_PlayerInventory.BPC_PlayerInventory_C"))
  (Utilities|IsValid _returnvalue
    (:Is%20Valid
      (Variables|/Game/OpenRPG/InventorySystem/Blueprints/Components/BPC_PlayerInventory.BPC_PlayerInventory_C|SetNearbyStorage _returnvalue self)
      (Rendering|SetVisibility (Variables|Default|GetInteractWidget) true false) ; Makes the interact widget visible
    )))

(event OnComponentEndOverlap(InteractColision)
  (params (OverlappedComponent :type Primitive%20Component%20Object%20Reference) (OtherActor :type Actor%20Object%20Reference) (OtherComp :type Primitive%20Component%20Object%20Reference) (OtherBodyIndex :type Integer))
  (bind _returnvalue (Actor|GetComponentbyClass OtherActor "/Game/OpenRPG/InventorySystem/Blueprints/Components/BPC_PlayerInventory.BPC_PlayerInventory_C"))
  (bind _bpc_storage (Variables|Default|GetBPC_Storage))
  (Utilities|IsValid _returnvalue
    (:Is%20Valid
      (Variables|/Game/OpenRPG/InventorySystem/Blueprints/Components/BPC_PlayerInventory.BPC_PlayerInventory_C|SetNearbyStorage _returnvalue 0)
      (Rendering|SetVisibility (Variables|Default|GetInteractWidget) false false) ; Makes the interact widget unvisible
      (if (Default|HasBeenInitialized? (Variables|Default|GetBPC_Storage))
        (Default|SaveInventory _bpc_storage)
        (if (Default|IsWidgetVisible? _bpc_storage)
          (Default|ToggleWidgetVisibility (Variables|Default|GetBPC_Storage)))))))

(event EventBeginPlay
  (bind _aswb_demo_interact_text (Utilities|Casting|CastToWB_DemoInteractText (UserInterface|GetUserWidgetObject (Variables|Default|GetInteractWidget)))) ; Get the widget from the component
  (bind _output_get (Variables|Default|SetWB_InteractText _aswb_demo_interact_text))
  (Default|Initialize _output_get "Storage" "O")
  (Rendering|SetVisibility (Variables|Default|GetInteractWidget) false false) ; Makes the interact widget visible
)

(event EventOnInteract
  (if (Default|HasBeenInitialized? (Variables|Default|GetBPC_Storage))
    _
    (else
      (Default|Initialize (Variables|Default|GetBPC_Storage))))
  (Default|ToggleWidgetVisibility (Variables|Default|GetBPC_Storage))
  (Default|UpdateContainerWidget (Variables|Default|GetBPC_Storage)))

(fn ConstructionScript
  (Components|Sphere|SetSphereRadius (Variables|Default|GetInteractColision) (Variables|Default|GetInteractRadius) true)
  (Components|StaticMesh|SetStaticMesh (Variables|Default|GetMesh) (Variables|Default|GetStorageMesh)))