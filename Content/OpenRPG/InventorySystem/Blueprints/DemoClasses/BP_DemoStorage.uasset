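; Demo storage container actor with its own inventory component, which the player opens within an interaction sphere.
; Overlap registers it with the player's BPC_PlayerInventory and shows a prompt; OnInteract initializes or toggles the storage UI.
; Slot clicks transfer items to the player; drops accept player items or rearrange storage via Shift-split, falling back to stack merge, then swap.
; The inventory saves on close, while construction applies configurable mesh and radius.
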(event OnSlotClicked(BPC_Inventory)
  (params (SlotIndex :type Integer))
  (bind _success_ (Default|TransferItem (Variables|Default|GetBPC_Inventory) (Variables|Default|GetPlayerInventory) -1 SlotIndex))
  (if _success_
    (Development|PrintString "Item Transfered Successfully")))

(event OnComponentBeginOverlap(InteractColision)
  (params (OverlappedComponent :type Primitive%20Component%20Object%20Reference) (OtherActor :type Actor%20Object%20Reference) (OtherComp :type Primitive%20Component%20Object%20Reference) (OtherBodyIndex :type Integer) (bFromSweep :type Boolean) (SweepResult :type Hit%20Result%20Structure%20%28by%20ref%29))
  (bind _returnvalue (Actor|GetComponentbyClass OtherActor "/Game/OpenRPG/InventorySystem/Blueprints/Components/BPC_PlayerInventory.BPC_PlayerInventory_C"))
  (Utilities|IsValid _returnvalue
    (:Is%20Valid
      (bind _output_get (Variables|Default|SetPlayerInventory _returnvalue))
      (Default|SetStorageActor _output_get self)
      (Rendering|SetVisibility (Variables|Default|GetInteractWidget) true false) ; Makes the interact widget visible
    )))

(event OnComponentEndOverlap(InteractColision)
  (params (OverlappedComponent :type Primitive%20Component%20Object%20Reference) (OtherActor :type Actor%20Object%20Reference) (OtherComp :type Primitive%20Component%20Object%20Reference) (OtherBodyIndex :type Integer))
  (bind _returnvalue (Actor|GetComponentbyClass OtherActor "/Game/OpenRPG/InventorySystem/Blueprints/Components/BPC_PlayerInventory.BPC_PlayerInventory_C"))
  (Utilities|IsValid _returnvalue
    (:Is%20Valid
      (Default|SetStorageActor _returnvalue)
      (Variables|Default|SetPlayerInventory 0)
      (Rendering|SetVisibility (Variables|Default|GetInteractWidget) false false) ; Makes the interact widget unvisible
    )))

(event OnInventoryClosed(BPC_Inventory)
  (Default|SaveInventory (Variables|Default|GetBPC_Inventory)))

(event OnReceiveSlotDrop(BPC_Inventory)
  (params (DroppedSlot :type Object%20Object%20Reference) (DroppedIndex :type Integer))
  (CallFunction|HandleSlotDrop DroppedSlot DroppedIndex))

(event Custom|OnInteract
  (if (Variables|/Game/OpenRPG/InventorySystem/Blueprints/Components/BPC_Inventory.BPC_Inventory_C|GetInitialized? (Variables|Default|GetBPC_Inventory))
    (Default|ToggleWidgetVisibility (Variables|Default|GetBPC_Inventory))
    (else
      (Default|Initialize (Variables|Default|GetBPC_Inventory)))))

(event EventBeginPlay
  (bind _aswb_interact_text (Utilities|Casting|CastToWB_InteractText (UserInterface|GetUserWidgetObject (Variables|Default|GetInteractWidget)))) ; Get the widget from the component
  (bind _output_get (Variables|Default|SetWB_InteractText _aswb_interact_text))
  (Default|Initialize _output_get "Storage" "O")
  (Rendering|SetVisibility (Variables|Default|GetInteractWidget) false false) ; Makes the interact widget visible
)

(fn ConstructionScript
  (Components|Sphere|SetSphereRadius (Variables|Default|GetInteractColision) (Variables|Default|GetInteractRadius) true)
  (Components|StaticMesh|SetStaticMesh (Variables|Default|GetMesh) (Variables|Default|GetStorageMesh)))

(fn HandleSlotDrop
  (params (DroppedSlot :type Object%20Object%20Reference) (DroppedIndex :type Integer))
  (LocalVariables|SetLocalIndex DroppedIndex)
  (bind _aswb_item_container_slot (Utilities|Casting|CastToWB_ItemContainerSlot DroppedSlot)
    (:then
      (bind _output_get (LocalVariables|SetLocalItemContainerSlot _aswb_item_container_slot))
      (if (!= _output_get (Utilities|Array|Get(acopy) (Variables|/Game/OpenRPG/InventorySystem/Widgets/WB_Inventory.WB_Inventory_C|GetSlots (Variables|/Game/OpenRPG/InventorySystem/Blueprints/Components/BPC_Inventory.BPC_Inventory_C|GetInventoryWidget (Variables|Default|GetBPC_Inventory))) (LocalVariables|GetLocalIndex)))
        (if (Variables|/Game/OpenRPG/InventorySystem/Widgets/WB_ItemContainerSlot.WB_ItemContainerSlot_C|GetInPlayerInventory? (LocalVariables|GetLocalItemContainerSlot))
          (Default|TransferItem (Variables|/Game/OpenRPG/InventorySystem/Widgets/WB_ItemContainerSlot.WB_ItemContainerSlot_C|GetInventoryComponent (LocalVariables|GetLocalItemContainerSlot)) (Variables|Default|GetBPC_Inventory) (LocalVariables|GetLocalIndex) (Variables|/Game/OpenRPG/InventorySystem/Widgets/WB_ItemContainerSlot.WB_ItemContainerSlot_C|GetSlotIndex (LocalVariables|GetLocalItemContainerSlot)))
          (return)
          (else
            (if (Variables|/Game/OpenRPG/InventorySystem/Widgets/WB_Inventory.WB_Inventory_C|GetShiftKeyDown? (Variables|/Game/OpenRPG/InventorySystem/Blueprints/Components/BPC_Inventory.BPC_Inventory_C|GetInventoryWidget (Variables|Default|GetBPC_Inventory)))
              (bind _success_ (Default|SplitStack (Variables|Default|GetBPC_Inventory) (Variables|/Game/OpenRPG/InventorySystem/Widgets/WB_ItemContainerSlot.WB_ItemContainerSlot_C|GetSlotIndex (LocalVariables|GetLocalItemContainerSlot)) (/ (Variables|/Game/OpenRPG/InventorySystem/Widgets/WB_ItemContainerSlot.WB_ItemContainerSlot_C|GetAmount (LocalVariables|GetLocalItemContainerSlot)) (Variables|/Game/OpenRPG/InventorySystem/Blueprints/Components/BPC_Inventory.BPC_Inventory_C|GetSplitDivideAmount (Variables|Default|GetBPC_Inventory))) (LocalVariables|GetLocalIndex)))
              (if _success_
                (return)
                (else
                  _)))
            (bind _success__2 (Default|AddAmountfromIndextoIndex (Variables|Default|GetBPC_Inventory) (Variables|/Game/OpenRPG/InventorySystem/Widgets/WB_ItemContainerSlot.WB_ItemContainerSlot_C|GetSlotIndex (LocalVariables|GetLocalItemContainerSlot)) (LocalVariables|GetLocalIndex)))
            (if _success__2
              (return)
              (else
                (Default|SwapItems (Variables|Default|GetBPC_Inventory) (Variables|/Game/OpenRPG/InventorySystem/Widgets/WB_ItemContainerSlot.WB_ItemContainerSlot_C|GetSlotIndex (LocalVariables|GetLocalItemContainerSlot)) (LocalVariables|GetLocalIndex))
                (return)))))))
    (:CastFailed
      (return))))