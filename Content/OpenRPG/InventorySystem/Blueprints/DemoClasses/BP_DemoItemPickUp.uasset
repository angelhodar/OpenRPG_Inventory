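; Demo world pickup actor for an inventory system that adds an item and amount to the player's inventory on interaction.
; The construction script looks up the item ID in DT_Items to set mesh, material, scale and interaction radius.
; Sphere overlaps register it as a nearby item with the player's inventory component and toggle a name-and-amount prompt widget.
; On interact, it unregisters and destroys itself only if adding succeeds.
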(event OnComponentBeginOverlap(InteractColisionRadius)
  (params (OverlappedComponent :type Primitive%20Component%20Object%20Reference) (OtherActor :type Actor%20Object%20Reference) (OtherComp :type Primitive%20Component%20Object%20Reference) (OtherBodyIndex :type Integer) (bFromSweep :type Boolean) (SweepResult :type Hit%20Result%20Structure%20%28by%20ref%29))
  (bind _returnvalue (Actor|GetComponentbyClass OtherActor "/Game/OpenRPG/InventorySystem/Blueprints/Components/BPC_PlayerInventory.BPC_PlayerInventory_C"))
  (Utilities|IsValid _returnvalue
    (:Is%20Valid
      (Default|AddNearbyItem _returnvalue self)
      (Rendering|SetVisibility (Variables|Default|GetInteractWidget) true false) ; Makes the interact widget visible
    )))

(event OnComponentEndOverlap(InteractColisionRadius)
  (params (OverlappedComponent :type Primitive%20Component%20Object%20Reference) (OtherActor :type Actor%20Object%20Reference) (OtherComp :type Primitive%20Component%20Object%20Reference) (OtherBodyIndex :type Integer))
  (bind _returnvalue (Actor|GetComponentbyClass OtherActor "/Game/OpenRPG/InventorySystem/Blueprints/Components/BPC_PlayerInventory.BPC_PlayerInventory_C"))
  (Utilities|IsValid _returnvalue
    (:Is%20Valid
      (Default|RemoveNearbyItem _returnvalue self)
      (Rendering|SetVisibility (Variables|Default|GetInteractWidget) false false) ; Makes the interact widget unvisible
    )))

(event Custom|OnInteract
  (params (PlayerInventory :type BPC%20Player%20Inventory%20Object%20Reference))
  (bind _success_ (Default|AddIItem PlayerInventory (Variables|Default|GetItemID) (Variables|Default|GetAmount)))
  (if _success_ ; Not enough space?
    (Default|RemoveNearbyItem PlayerInventory self)
    (Actor|DestroyActor)))

(event EventBeginPlay
  (bind _aswb_interact_text (Utilities|Casting|CastToWB_InteractText (UserInterface|GetUserWidgetObject (Variables|Default|GetInteractWidget)))) ; Get the widget from the component
  (bind _output_get (Variables|Default|SetWB_InteractText _aswb_interact_text))
  (Default|Initialize _output_get (Utilities|Text|FormatText "{Name} x{Amount}" (Utilities|Text|ToText(Name) (Utilities|Struct|Breaks_ItemData (Variables|Default|GetItemData))) (Variables|Default|GetAmount)) "E")
  (CallFunction|SetVisualProperties)
  (Rendering|SetVisibility (Variables|Default|GetInteractWidget) false false) ; Makes the interact widget visible
)

(fn ConstructionScript
  (if (!= (Variables|Default|GetItemID) -1)
    (bind _returnvalue (Utilities|GetDataTableRow "/Game/OpenRPG/InventorySystem/Blueprints/Items/DataTables/DT_Items.DT_Items" (Utilities|String|StringToName (Utilities|String|ToString(Integer) (Variables|Default|GetItemID)))) ; Get the info from the data table
      (:then
        (Variables|Default|SetItemData _returnvalue)
        (CallFunction|SetVisualProperties)))))

(fn SetVisualProperties
  (bind _itemdata (Variables|Default|GetItemData))
  (bind _itemdata_2 (Variables|Default|GetItemData))
  (bind (_meshscale _interactradius) (Utilities|Struct|Breaks_ItemData _itemdata))
  (bind _worldmesh (Utilities|Struct|Breaks_ItemData _itemdata_2))
  (Components|StaticMesh|SetStaticMesh (Variables|Default|GetItemMesh) _worldmesh)
  (Rendering|Material|SetMaterial (Variables|Default|GetItemMesh) 0 (Rendering|Material|GetMaterial _worldmesh 0))
  (Transformation|SetWorldScale3D (Variables|Default|GetItemMesh) _meshscale)
  (Components|Sphere|SetSphereRadius (Variables|Default|GetInteractColisionRadius) _interactradius false))