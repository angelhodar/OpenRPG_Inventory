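; ItemsSave is an inventory save Blueprint that holds saved container items for the inventory system.
; It keeps a map keyed by save name, where each entry is a struct of the items and their slots-per-row layout.
; AddNewSavedItems writes an entry under a given name, and GetSavedItems looks one up, returning a found flag with the saved data.
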(fn AddNewSavedItems
  (params (SaveName :type String) (Items :type Array%20of%20S%20Inventory%20Item%20Structures) (SlotsPerRow :type Integer))
  (LocalVariables|SetLocalSaveName SaveName)
  (LocalVariables|SetLocalItems Items)
  (LocalVariables|SetLocalSlotsPerRow SlotsPerRow)
  (Utilities|Map|Add (Variables|Default|GetSavedContainerItems) (LocalVariables|GetLocalSaveName) (Utilities|Struct|Makes_SavedItems (LocalVariables|GetLocalSlotsPerRow) (LocalVariables|GetLocalItems)))
  (return))

(fn GetSavedItems
  (params (SaveName :type String))
  (bind _savedcontaineritems (Variables|Default|GetSavedContainerItems))
  (bind (_value _returnvalue) (Utilities|Map|Find _savedcontaineritems SaveName))
  (return _returnvalue _value))