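; BP_BaseLoot is the master class for loot items that a player opens from an inventory slot to receive their contents.
; UseItem calls ManageLoot, which looks up the item's loot row in DT_Loot and checks for inventory space.
; On success it removes one loot item, adds the contents through the inventory handler and fires OnItemUsed.
; Failures print a message, and the actor is destroyed either way.
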(event EventUseItem
  (params (Clicked%20Slot%20Index :type Integer) (PlayerController :type BP%20Custom%20Player%20Controller%20Object%20Reference))
  (|CallParentFunction Clicked%20Slot%20Index PlayerController)
  (bind _success_ (CallFunction|ManageLoot))
  (if _success_
    (CallFunction|OnItemUsed))
  (Actor|DestroyActor))

(fn ConstructionScript
  (|CallParentFunction))

(fn GetLootfromID
  (params (LootRowName :type Name))
  (bind _returnvalue (Utilities|GetDataTableRow "/Game/OpenRPG/InventorySystem/Blueprints/Items/DataTables/DT_Loot.DT_Loot" LootRowName)
    (:then
      (return (Utilities|Struct|Breaks_Loot _returnvalue)))
    (:RowNotFound
      (return 0))))

(fn ManageLoot
  (bind _itemdata (Variables|Default|GetItemData))
  (bind _lootdatarowname (Utilities|Struct|Breaks_ItemData _itemdata))
  (if (Utilities|Name|NotEqual(Name) _lootdatarowname "None")
    (LocalVariables|SetLocalLoot (CallFunction|GetLootfromID _lootdatarowname))
    (if (Default|CanAddItems? (Variables|/Game/OpenRPG/Shared/Blueprints/BP_CustomPlayerController.BP_CustomPlayerController_C|GetBPC_InventoryHandler (Variables|Default|GetPlayerController)) (LocalVariables|GetLocalLoot))
      (Default|RemoveAmountatIndex (Variables|/Game/OpenRPG/Shared/Blueprints/BP_CustomPlayerController.BP_CustomPlayerController_C|GetBPC_InventoryHandler (Variables|Default|GetPlayerController)) (Variables|Default|GetClickedSlotIndex) 1)
      (for _array_element (LocalVariables|GetLocalLoot)
        (Default|AddIItem(Public) (Variables|/Game/OpenRPG/Shared/Blueprints/BP_CustomPlayerController.BP_CustomPlayerController_C|GetBPC_InventoryHandler (Variables|Default|GetPlayerController)) (.ItemID (Utilities|Struct|Breaks_InventoryItem _array_element)) (.Amount (Utilities|Struct|Breaks_InventoryItem _array_element))))
      (return true)
      (else
        (Development|PrintString "Not enough space to open the loot!")
        (return false)))
    (else
      (Development|PrintString "Invalid loot row name")
      (return false))))