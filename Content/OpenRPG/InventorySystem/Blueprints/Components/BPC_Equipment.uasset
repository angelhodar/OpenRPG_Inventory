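; BPC_Equipment is an actor component that manages a player's equipped items, one slot per equipment type.
; Initialize checks the owner's interfaces, links the inventory component and equipment widget, then restores saved equipment.
; EquipItem reads DT_Equipment, sets the slot's skeletal mesh using master pose or socket attachment, and swaps occupied slots through the inventory.
; Unequipping returns or drops items, while SaveGame objects persist the slot array.
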(event Custom|Initialize
  (params (EquipmentWidget :type WB%20Equipment%20Object%20Reference))
  (Variables|Default|SetEquipmentWidget EquipmentWidget)
  (CallFunction|SetupEquipmentArray)
  (if (Utilities|DoesObjectImplementInterface (Components|GetOwner) "/Game/OpenRPG/InventorySystem/Blueprints/Interfaces/BPI_Equipment.BPI_Equipment_C")
    (if (Utilities|DoesObjectImplementInterface (Components|GetOwner) "/Game/OpenRPG/InventorySystem/Blueprints/Interfaces/BPI_PlayerInventory.BPI_PlayerInventory_C")
      (bind _inventorycomponent (Class|BPIPlayerInventory|GetPlayerInventoryComponent(Message) (Components|GetOwner)))
      (bind _output_get (Variables|Default|SetInventoryComponentReference _inventorycomponent))
      (Utilities|IsValid _output_get
        (:Is%20Valid
          (Utilities|IsValid (Variables|Default|GetEquipmentWidget)
            (:Is%20Valid
              _)
            (:Is%20Not%20Valid
              (bind _returnvalue (UserInterface|CreateWidget "/Game/OpenRPG/InventorySystem/Widgets/WB_Equipment.WB_Equipment_C"))
              (Variables|Default|SetEquipmentWidget _returnvalue)
              (UserInterface|Viewport|AddtoViewport (Variables|Default|GetEquipmentWidget) (Variables|Default|GetZOrder))
              (Class|UserWidget|SetPositioninViewport (Variables|Default|GetEquipmentWidget) (/ (Viewport|GetViewportSize) 2.0) true)))
          (Default|Initialize (Variables|Default|GetEquipmentWidget) self (Variables|Default|GetInventoryComponentReference))
          (CallFunction|LoadEquipment)
          (Development|PrintString "Your BPC_Equipment is configured successfully!!!" true true "(R=1.000000,G=0.086574,B=0.000000,A=1.000000)" 1e+01))
        (:Is%20Not%20Valid
          (Development|PrintString "Error: The function GetPlayerInventoryComponent from BPI_Inventory interface in your player returns a not valid reference" true true "(R=1.000000,G=0.086574,B=0.000000,A=1.000000)" 1e+01)))
      (else
        (Development|PrintString "Error: Your player doesnt implement the required BPI_Inventory interface" true true "(R=1.000000,G=0.086574,B=0.000000,A=1.000000)" 1e+01)))
    (else
      (Development|PrintString "Error: Your player doesnt implement the required BPI_Equipment interface" true true "(R=1.000000,G=0.086574,B=0.000000,A=1.000000)" 1e+01))))

(event Custom|UpdateEquipmentSlot
  (params (Slot :type e_EquipmentType%20Enum :default "NewEnumerator0"))
  (Default|Update (CallFunction|GetEquipmentSlotWidget Slot)))

(fn GetEquipmentDatafromRow
  (params (RowName :type Name))
  (bind _returnvalue (Utilities|GetDataTableRow "/Game/OpenRPG/InventorySystem/Blueprints/Items/DataTables/DT_Equipment.DT_Equipment" RowName)
    (:then
      (return _returnvalue))
    (:RowNotFound
      (return ""))))

(fn GetEquipmentSlotWidget
  (params (SlotType :type e_EquipmentType%20Enum :default "NewEnumerator0"))
  (LocalVariables|SetLocalType SlotType)
  (bind _array_element (Utilities|Array|ForEachLoopwithBreak (Variables|/Game/OpenRPG/InventorySystem/Widgets/WB_Equipment.WB_Equipment_C|GetSlots (Variables|Default|GetEquipmentWidget)) :!label _label)
    (:LoopBody
      (if (Utilities|Enum|Equal(Enum) (Variables|/Game/OpenRPG/InventorySystem/Widgets/WB_EquipmentSlot.WB_EquipmentSlot_C|GetType _array_element) (LocalVariables|GetLocalType))
        (LocalVariables|SetLocalSlotWidget _array_element)
        (goto _label Break)))
    (:Completed
      (return (LocalVariables|GetLocalSlotWidget)))))

(fn GetIteminSlot
  (params (SlotType :type e_EquipmentType%20Enum :default "NewEnumerator0"))
  (LocalVariables|SetLocalSlot SlotType)
  (bind _array_element (Utilities|Array|ForEachLoopwithBreak (Variables|Default|GetEquipment) :!label _label)
    (:LoopBody
      (if (Utilities|Enum|Equal(Enum) (.Type (Utilities|Struct|Breaks_EquipmentItem _array_element)) (LocalVariables|GetLocalSlot))
        (LocalVariables|SetLocalItemID (.ItemID (Utilities|Struct|Breaks_EquipmentItem _array_element))) ; The default value of this variable is -1
        (goto _label Break)))
    (:Completed
      (return (LocalVariables|GetLocalItemID)))))

(fn SetNewEquipmentItem
  (params (ItemID :type Integer) (SlotType :type e_EquipmentType%20Enum :default "NewEnumerator0"))
  (LocalVariables|SetLocalItemID ItemID)
  (LocalVariables|SetLocalSlot SlotType)
  (bind (_array_element _array_index) (Utilities|Array|ForEachLoopwithBreak (Variables|Default|GetEquipment) :!label _label)
    (:LoopBody
      (if (Utilities|Enum|Equal(Enum) (Utilities|Struct|Breaks_EquipmentItem _array_element) (LocalVariables|GetLocalSlot))
        (Utilities|Array|SetArrayElem (Variables|Default|GetEquipment) _array_index (Utilities|Struct|Makes_EquipmentItem (LocalVariables|GetLocalItemID) (LocalVariables|GetLocalSlot)) true)
        (goto _label Break)))
    (:Completed
      (return))))

(fn EquipItem
  (params (Item :type Integer) (FromInventorySlot :type Integer))
  ;[0.08879 0.8399 1] This part of the code just extracts the necessary data and set it, giving warnings when something is not correctly set.
  (LocalVariables|SetLocalItemID Item)
  (LocalVariables|SetLocalClickedInventorySlot FromInventorySlot)
  (Utilities|IsValid (Variables|Default|GetInventoryComponentReference)
    (:Is%20Valid
      (bind _mesh (Class|BPIEquipment|GetPlayerMesh(Message) (Components|GetOwner)))
      (bind _output_get (LocalVariables|SetLocalPlayerMesh _mesh))
      (Utilities|IsValid _output_get
        (:Is%20Valid
          (bind _meshcomponent (Class|BPIEquipment|GetEquipmentMeshComponentbyType(Message) (Components|GetOwner) (LocalVariables|GetLocalSlotType)))
          (bind _output_get_2 (LocalVariables|SetLocalMeshComponent _meshcomponent)) ; We get the mesh component of the player that we are going to update
          (Utilities|IsValid _output_get_2
            (:Is%20Valid
              (bind _output_get_3 (LocalVariables|SetLocalItemData (Default|GetItemDatafromID (Variables|Default|GetInventoryComponentReference) (LocalVariables|GetLocalItemID))))
              (if (Utilities|Name|NotEqual(Name) (Utilities|Struct|Breaks_ItemData _output_get_3) "None")
                (bind _output_get_4 (LocalVariables|SetLocalEquipmentData (CallFunction|GetEquipmentDatafromRow (Utilities|Struct|Breaks_ItemData _output_get_3))))
                (bind _output_get_5 (LocalVariables|SetLocalSlotType (Utilities|Struct|Breaks_EquipmentData _output_get_4)))
                (bind _output_get_6 (LocalVariables|SetLocalEquippedItemID (CallFunction|GetIteminSlot _output_get_5))) ; We extract the ID of the item that could be equipped when we want to equip in that slot
                (if (== _output_get_6 -1) ; Is the slot empty?
                  ;[1 0.91 0.07485] This part is responsible of the visual equipment, it updates the player pawn with the skeletal mesh of the item that we are going to equip
                  (Utilities|IsValid (Utilities|Struct|Breaks_EquipmentData (LocalVariables|GetLocalEquipmentData)) ; If the mesh isnt valid we skip the visual logic part
                    (:Is%20Valid
                      (Class|SkinnedMeshComponent|SetSkeletalMesh (LocalVariables|GetLocalMeshComponent) (Utilities|Struct|Breaks_EquipmentData (LocalVariables|GetLocalEquipmentData)) true) ; We set the mesh of that component to the one in the equipment data
                      (if (Utilities|Name|Equal(Name) (Utilities|Struct|Breaks_EquipmentData (LocalVariables|GetLocalEquipmentData)) "None") ; If we want to attach the component in a particular bone with custom transform this will have a valid value (only recommended for weapons)
                        (Class|SkinnedMeshComponent|SetMasterPoseComponent (LocalVariables|GetLocalMeshComponent) (LocalVariables|GetLocalPlayerMesh)) ; If the skeletal mesh has the same skeleton as our player, this function will make it to fit it
                        (else
                          (Transformation|AttachComponentToComponent (LocalVariables|GetLocalMeshComponent) (LocalVariables|GetLocalPlayerMesh) (Utilities|Struct|Breaks_EquipmentData (LocalVariables|GetLocalEquipmentData)) "KeepRelative" "KeepRelative" "KeepRelative" true)
                          (Transformation|SetRelativeTransform (LocalVariables|GetLocalMeshComponent) (Utilities|Struct|Breaks_EquipmentData (LocalVariables|GetLocalEquipmentData)) false false))))
                    (:Is%20Not%20Valid
                      _))
                  (CallFunction|SetNewEquipmentItem (LocalVariables|GetLocalItemID) (LocalVariables|GetLocalSlotType))
                  (CallFunction|UpdateEquipmentSlot (LocalVariables|GetLocalSlotType))
                  (if (== (LocalVariables|GetLocalClickedInventorySlot) -1) ; If false it means the equip comes from an inventory slot
                    _
                    (else
                      (Default|RemoveIndexAmount (Variables|Default|GetInventoryComponentReference) (LocalVariables|GetLocalClickedInventorySlot) 1) ; So we remove the item in that slot, if not we would see it in the equipment slot and in the inventory
                    ))
                  (Default|CallOnItemEquipped (LocalVariables|GetLocalItemID) (LocalVariables|GetLocalSlotType))
                  (return)
                  (else
                    ;[1 0.09225 0.142] This part of the code makes a swap between the item that we know its already equipped and the one that we want to equip
                    (Default|RemoveIndexAmount (Variables|Default|GetInventoryComponentReference) (LocalVariables|GetLocalClickedInventorySlot) 1) ; First we clean the slot of the item that we are going to equip (we have it stored in the LocalItemID variable)
                    (CallFunction|UnequipItem (LocalVariables|GetLocalSlotType) (LocalVariables|GetLocalClickedInventorySlot) false)
                    (CallFunction|EquipItem (LocalVariables|GetLocalItemID) -1)
                    (return)))
                (else
                  (Development|PrintString "Invalid row name to get the equipment data")
                  (return))))
            (:Is%20Not%20Valid
              (Development|PrintString "Error: The function GetEquipmentMeshComponentByType in your player isnt implemented correctly, its returning a not valid mesh component" true true "(R=0.000000,G=0.660000,B=1.000000,A=1.000000)" 2e+01)
              (return))))
        (:Is%20Not%20Valid
          (Development|PrintString "Error: The function GetPlayerMesh in your player isnt implemented correctly, its returning a not valid mesh component")
          (return))))
    (:Is%20Not%20Valid
      (Development|PrintString "Error: The InventoryComponent reference in the EquipmentComponent is not valid!" true true "(R=0.000000,G=0.660000,B=1.000000,A=1.000000)" 8.0)
      (return))))

(fn UnequipItem
  (params (SlotType :type e_EquipmentType%20Enum :default "NewEnumerator0") (ToSpecificInventoryIndex :type Integer) (Drop? :type Boolean))
  (LocalVariables|SetLocalSlotType SlotType)
  (LocalVariables|SetLocalSpecificIndex ToSpecificInventoryIndex)
  (LocalVariables|SetLocalDrop Drop?)
  (Utilities|IsValid (Variables|Default|GetInventoryComponentReference)
    (:Is%20Valid
      (bind _meshcomponent (Class|BPIEquipment|GetEquipmentMeshComponentbyType(Message) (Components|GetOwner) (LocalVariables|GetLocalSlotType)))
      (bind _output_get (LocalVariables|SetLocalMeshComponent _meshcomponent)) ; We get the mesh component of the player that we are going to update
      (Utilities|IsValid _output_get
        (:Is%20Valid
          (LocalVariables|SetLocalEquippedItemID (CallFunction|GetIteminSlot (LocalVariables|GetLocalSlotType))) ; We get the current equipped item in the slot
          (if (LocalVariables|GetLocalDrop)
            (Default|DropItem (Variables|Default|GetInventoryComponentReference) (LocalVariables|GetLocalEquippedItemID) 1)
            (elif (!= (LocalVariables|GetLocalSpecificIndex) -1) ; If true it means we have to unequip to a specifil inventory index (we are dragging from the equipment slot to an inventory slot)
              (if (Default|IsSlotEmpty? (Variables|Default|GetInventoryComponentReference) (LocalVariables|GetLocalSpecificIndex)) ; If the slot is empty it means we can drop the item in the inventory slot
                (Default|AddItemtoIndex (Variables|Default|GetInventoryComponentReference) (LocalVariables|GetLocalEquippedItemID) 1 (LocalVariables|GetLocalSpecificIndex)) ; We add it
                (else
                  (Development|PrintString "Drop index has already an item")
                  (return false)))
              (else
                (bind _success_ (Default|AddIItem (Variables|Default|GetInventoryComponentReference) (LocalVariables|GetLocalEquippedItemID) 1)) ; We unequip in the first emty slot
                (if _success_
                  _
                  (else
                    (Development|PrintString "Error while unequipping the item, maybe not enough space in inventory")
                    (return false))))))
          (Class|SkinnedMeshComponent|SetSkeletalMesh (LocalVariables|GetLocalMeshComponent) 0 true) ; Resets the visual equipment, it simulates that we unequipped the item
          (CallFunction|SetNewEquipmentItem -1 (LocalVariables|GetLocalSlotType))
          (CallFunction|UpdateEquipmentSlot (LocalVariables|GetLocalSlotType))
          (Default|CallOnItemUnequipped (LocalVariables|GetLocalEquippedItemID) (LocalVariables|GetLocalSlotType) (LocalVariables|GetLocalDrop))
          (return true))
        (:Is%20Not%20Valid
          (Development|PrintString "Error: The function GetEquipmentMeshComponentByType in your player isnt implemented correctly, its returning a not valid mesh component" true true "(R=0.000000,G=0.660000,B=1.000000,A=1.000000)" 2e+01)
          (return false))))
    (:Is%20Not%20Valid
      (Development|PrintString "Error: The InventoryComponent reference in the EquipmentComponent is not valid!")
      (return false))))

(fn ToggleEquipmentVisibility
  (Widget|SetVisibility (Variables|Default|GetEquipmentWidget) (select (Widget|IsVisible (Variables|Default|GetEquipmentWidget)) "Hidden" "Visible"))
  (return))

(fn SaveEquipment
  (Utilities|IsValid (Variables|Default|GetSaveEquipmentObject)
    (:Is%20Valid
      _)
    (:Is%20Not%20Valid
      (bind _returnvalue (SaveGame|CreateSaveGameObject "/Game/OpenRPG/InventorySystem/Blueprints/SaveClasses/EquipmentSave.EquipmentSave_C"))
      (Variables|Default|SetSaveEquipmentObject _returnvalue)))
  (Variables|/Game/OpenRPG/InventorySystem/Blueprints/SaveClasses/EquipmentSave.EquipmentSave_C|SetSavedEquipment (Variables|Default|GetSaveEquipmentObject) (Variables|Default|GetEquipment))
  (SaveGame|SaveGametoSlot (Variables|Default|GetSaveEquipmentObject) (Variables|Default|GetSaveEquipmentSlotName))
  (Default|CallOnEquipmentSaved)
  (return))

(fn LoadEquipment
  (bind _returnvalue (SaveGame|DoesSaveGameExist (Variables|Default|GetSaveEquipmentSlotName)))
  (if _returnvalue
    (Utilities|IsValid (Variables|Default|GetSaveEquipmentObject)
      (:Is%20Valid
        _)
      (:Is%20Not%20Valid
        (bind _returnvalue_2 (SaveGame|LoadGamefromSlot (Variables|Default|GetSaveEquipmentSlotName)))
        (bind _asequipment_save (Utilities|Casting|CastToEquipmentSave _returnvalue_2)
          (:then
            (Variables|Default|SetSaveEquipmentObject _asequipment_save))
          (:CastFailed
            (return false)))))
    (for _array_element (Variables|/Game/OpenRPG/InventorySystem/Blueprints/SaveClasses/EquipmentSave.EquipmentSave_C|GetSavedEquipment (Variables|Default|GetSaveEquipmentObject))
      (if (!= (Utilities|Struct|Breaks_EquipmentItem _array_element) -1)
        (CallFunction|EquipItem (Utilities|Struct|Breaks_EquipmentItem _array_element) -1)))
    (Default|CallOnEquipmentLoaded)
    (return true)
    (else
      (return false))))

(fn SetupEquipmentArray
  (bind _enumvalue (|ForEache_EquipmentType)
    (:LoopBody
      (Utilities|Array|Add (Variables|Default|GetEquipment) (Utilities|Struct|Makes_EquipmentItem -1 _enumvalue)))
    (:then
      (return))))