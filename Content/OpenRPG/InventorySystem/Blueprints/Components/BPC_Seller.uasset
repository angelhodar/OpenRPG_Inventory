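; BPC_Seller is a vendor inventory component through which the player buys and sells items.
; Clicking a slot calls BuyItem, which charges item value times amount, adds a copy to the player inventory (first fit or given index), and refunds if adding fails.
; Vendor stock is not decremented on purchase.
; Dropping a slot from one specific container type, apparently the player's, calls SellItem on the player inventory.
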(event EventOnSlotClicked
  (params (ClickedIndex :type Integer) (QuickActionEnabled? :type Boolean))
  ;[1 0.03646 0.1158] Override On Slot Clicked: Just calls the function BuyItem
  (CallFunction|BuyItem ClickedIndex -1))

(event EventOnSlotDrop
  (params (DroppedSlot :type Object%20Object%20Reference) (DroppedIndex :type Integer))
  ;[0.02391 0.00239 1] Override On Slot Clicked
  (CallFunction|HandleSlotDrop DroppedSlot DroppedIndex))

(fn BuyItem
  (params (Index :type Integer) (ToSpecificPlayerIndex :type Integer))
  (LocalVariables|SetLocalIndex Index)
  (LocalVariables|SetLocalSpecificPlayerIndex ToSpecificPlayerIndex)
  (LocalVariables|SetLocalItemCost (* (Utilities|Struct|Breaks_ItemData (CallFunction|GetItemDatafromID (.ItemID (Utilities|Struct|Breaks_InventoryItem (CallFunction|GetItematIndex (LocalVariables|GetLocalIndex)))))) (.Amount (Utilities|Struct|Breaks_InventoryItem (CallFunction|GetItematIndex (LocalVariables|GetLocalIndex))))))
  (bind _output_get (LocalVariables|SetLocalPlayerInventory (CallFunction|GetPlayerInventory)))
  (bind _success_ (Default|AddMoney _output_get (* (LocalVariables|GetLocalItemCost) -1)))
  (if _success_
    (if (== (LocalVariables|GetLocalSpecificPlayerIndex) -1)
      (bind _success__2 (Default|AddIItem (LocalVariables|GetLocalPlayerInventory) (CallFunction|GetItematIndex (LocalVariables|GetLocalIndex))))
      (if _success__2
        _
        (else
          (Default|AddMoney (LocalVariables|GetLocalPlayerInventory) (LocalVariables|GetLocalItemCost) :!label _label)
          (return)))
      (else
        (bind _success__3 (Default|AddItemtoIndex (LocalVariables|GetLocalPlayerInventory) (CallFunction|GetItematIndex (LocalVariables|GetLocalIndex)) (LocalVariables|GetLocalSpecificPlayerIndex)))
        (if _success__3
          _
          (else
            (goto _label)))))
    (return)
    (else
      (Development|PrintString "You dont have enough money to buy the item")
      (return))))

(fn HandleSlotDrop
  (params (DroppedSlot :type Object%20Object%20Reference) (DroppedIndex :type Integer))
  (LocalVariables|SetLocalDroppedSlot DroppedSlot)
  (LocalVariables|SetLocalDroppedIndex DroppedIndex)
  (bind _aswb_item_container_slot (Utilities|Casting|CastToWB_ItemContainerSlot (LocalVariables|GetLocalDroppedSlot))
    (:then
      (bind _output_get (LocalVariables|SetLocalItemSlot _aswb_item_container_slot))
      (if (Utilities|Enum|Equal(Enum) (Variables|/Game/OpenRPG/InventorySystem/Widgets/WB_ItemContainerSlot.WB_ItemContainerSlot_C|GetContainer _output_get) "NewEnumerator0")
        (bind _output_get_2 (LocalVariables|SetLocalPlayerInventory (CallFunction|GetPlayerInventory)))
        (Default|SellItem _output_get_2 (Variables|/Game/OpenRPG/InventorySystem/Widgets/WB_ItemContainerSlot.WB_ItemContainerSlot_C|GetSlotIndex (LocalVariables|GetLocalItemSlot)))
        (return)
        (else
          (return))))
    (:CastFailed
      (return))))