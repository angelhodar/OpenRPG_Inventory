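; Player inventory component that extends item container behavior with money, item use, selling and saved money.
; Slot clicks either use the item, by spawning its class actor to run the logic, or quick-transfer it to an open nearby storage or seller.
; Drops route by source: split, stack or swap within the inventory, transfer from storage, buy from seller, or unequip.
; It also tracks nearby items and forwards interaction to nearby storage and sellers.
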(event Custom|OpenStorage
  ;[0.1548 1 0.02316] Interaction with storage and seller actors
  (Utilities|IsValid (Variables|Default|GetNearbyStorage)
    (:Is%20Valid
      (Class|BPIWorldInteraction|OnInteract(Message) (Variables|Default|GetNearbyStorage)))))

(event Custom|OpenSeller
  ;[0.1548 1 0.02316] Interaction with storage and seller actors
  (Utilities|IsValid (Variables|Default|GetNearbySeller)
    (:Is%20Valid
      (Class|BPIWorldInteraction|OnInteract(Message) (Variables|Default|GetNearbySeller)))))

(event EventOnSlotDrop
  (params (DroppedSlot :type Object%20Object%20Reference) (DroppedIndex :type Integer))
  ;[0.02391 0.00239 1] Override slot drop
  (CallFunction|HandleSlotDrop DroppedSlot DroppedIndex))

(event EventOnSaveExtraData
  ;[1 0.7938 0.03439] Override of the save/load extra data events to manage the SavedMoney variable in ItemsSave class
  (Variables|/Game/OpenRPG/InventorySystem/Blueprints/Save/ItemsSave.ItemsSave_C|SetSavedMoney (Variables|Default|GetInventorySaveObject) (Variables|Default|GetCurrentMoney)))

(event EventOnLoadExtraData
  ;[1 0.7938 0.03439] Override of the save/load extra data events to manage the SavedMoney variable in ItemsSave class
  (Variables|Default|SetCurrentMoney (Variables|/Game/OpenRPG/InventorySystem/Blueprints/Save/ItemsSave.ItemsSave_C|GetSavedMoney (Variables|Default|GetInventorySaveObject))))

(event EventOnSlotClicked
  (params (ClickedIndex :type Integer))
  ;[1 0.03646 0.1158] Overriden event to use an item when a ui slot is clicked
  (if (Variables|/Game/OpenRPG/InventorySystem/Widgets/WB_ItemsContainerGrid.WB_ItemsContainerGrid_C|GetQuickActionKeyDown? (Variables|Default|GetContainerGridWidget))
    (CallFunction|HandleQuickAction ClickedIndex)
    (else
      (CallFunction|UseItem ClickedIndex))))

(fn CanUseItem?
  (params (Index :type Integer))
  (LocalVariables|SetLocalIndex Index)
  (LocalVariables|SetLocalPlayerLevel (CallFunction|GetPlayerLevel))
  (return (Math|Boolean|ANDBoolean (not (CallFunction|IsSlotEmpty? (LocalVariables|GetLocalIndex))) (Utilities|Enum|NotEqual(Enum) (Utilities|Struct|Breaks_ItemData (CallFunction|GetItemDatafromID (Utilities|Struct|Breaks_InventoryItem (CallFunction|GetItematIndex (LocalVariables|GetLocalIndex))))) "NewEnumerator2") (Utilities|Enum|NotEqual(Enum) (Utilities|Struct|Breaks_ItemData (CallFunction|GetItemDatafromID (Utilities|Struct|Breaks_InventoryItem (CallFunction|GetItematIndex (LocalVariables|GetLocalIndex))))) "NewEnumerator3") (>= (LocalVariables|GetLocalPlayerLevel) 0))))

(fn AddNearbyItem
  (params (NearbyActor :type BP%20World%20Item%20Object%20Reference))
  (bind _output_get (LocalVariables|SetLocalNearby NearbyActor))
  (if (Utilities|Array|ContainsItem (Variables|Default|GetNearbyItems) _output_get)
    (return)
    (else
      (Utilities|Array|Add (Variables|Default|GetNearbyItems) (LocalVariables|GetLocalNearby))
      (return))))

(fn RemoveNearbyItem
  (params (NearbyActor :type BP%20World%20Item%20Object%20Reference))
  (bind _output_get (LocalVariables|SetLocalNearby NearbyActor))
  (if (Utilities|Array|ContainsItem (Variables|Default|GetNearbyItems) _output_get)
    (Utilities|Array|RemoveItem (Variables|Default|GetNearbyItems) (LocalVariables|GetLocalNearby))
    (return)
    (else
      (return))))

(fn AddMoney
  (params (Amount :type Integer))
  (bind _output_get (LocalVariables|SetLocalAmount Amount))
  (bind _output_get_2 (LocalVariables|SetLocalNewAmount (+ _output_get (Variables|Default|GetCurrentMoney))))
  (if (and (<= _output_get_2 (Variables|Default|GetMaxMoney)) (>= (LocalVariables|GetLocalNewAmount) 0)) ; Are we going to have more than the max money or below 0?
    (Variables|Default|SetCurrentMoney (LocalVariables|GetLocalNewAmount))
    (Default|CallOnMoneyReceived (LocalVariables|GetLocalAmount) (LocalVariables|GetLocalNewAmount))
    (return true)
    (else
      (return false))))

(fn SellItem
  (params (Index :type Integer))
  (LocalVariables|SetLocalIndex Index)
  (if (not (CallFunction|IsSlotEmpty? (LocalVariables|GetLocalIndex)))
    (LocalVariables|SetLocalItem (.ItemID (Utilities|Struct|Breaks_InventoryItem (CallFunction|GetItematIndex (LocalVariables|GetLocalIndex)))))
    (LocalVariables|SetLocalAmount (.Amount (Utilities|Struct|Breaks_InventoryItem (CallFunction|GetItematIndex (LocalVariables|GetLocalIndex)))))
    (if (Utilities|Enum|NotEqual(Enum) (.Type (Utilities|Struct|Breaks_ItemData (CallFunction|GetItemDatafromID (LocalVariables|GetLocalItem)))) "NewEnumerator2")
      (bind _output_get (LocalVariables|SetLocalBenefit (* (.Value (Utilities|Struct|Breaks_ItemData (CallFunction|GetItemDatafromID (LocalVariables|GetLocalItem)))) (LocalVariables|GetLocalAmount))))
      (bind _success_ (CallFunction|AddMoney _output_get))
      (if _success_
        (CallFunction|RemoveIndexAmount (LocalVariables|GetLocalIndex) (LocalVariables|GetLocalAmount))
        (return true)
        (else
          (return false)))
      (else
        (return false)))
    (else
      (return false))))

(fn UseItem
  (params (Index :type Integer))
  (bind _output_get (LocalVariables|SetLocalIndex Index))
  (if (CallFunction|CanUseItem? _output_get)
    (bind _output_get_2 (LocalVariables|SetLocalItemID (Utilities|Struct|Breaks_InventoryItem (CallFunction|GetItematIndex (LocalVariables|GetLocalIndex)))))
    (bind _output_get_3 (LocalVariables|SetLocalItemData (CallFunction|GetItemDatafromID _output_get_2)))
    (if (Utilities|IsValidClass (Utilities|Struct|Breaks_ItemData _output_get_3)) ; You could print some string if false
      (bind _returnvalue (Game|SpawnActorfromClass (Utilities|Struct|Breaks_ItemData _output_get_3) (Math|Transform|MakeTransform "0, 0, 0" "0, 0, 0" "1,1,1") "AlwaysSpawn" 0 (LocalVariables|GetLocalItemID) (LocalVariables|GetLocalItemData) self 0)) ; This will spawn the class associated with the item that contains all the logic that has to be excuted
      (Default|UseItem _returnvalue (LocalVariables|GetLocalIndex)) ; Starts the item logic execution based on its type
      (Default|CallOnItemUsed (LocalVariables|GetLocalItemID))
      (return true)
      (else
        (return false)))
    (else
      (return false))))

(fn HandleQuickAction
  (params (ClickedIndex :type Integer))
  (bind _nearbystorage (Variables|Default|GetNearbyStorage))
  (bind _nearbyseller (Variables|Default|GetNearbySeller))
  (bind _returnvalue (Actor|GetComponentbyClass _nearbyseller "/Game/OpenRPG/InventorySystem/Blueprints/Components/BPC_ItemsContainer.BPC_ItemsContainer_C"))
  (bind _returnvalue_2 (Actor|GetComponentbyClass _nearbystorage "/Game/OpenRPG/InventorySystem/Blueprints/Components/BPC_ItemsContainer.BPC_ItemsContainer_C"))
  (LocalVariables|SetLocalClickedSlot ClickedIndex)
  (Utilities|IsValid (Variables|Default|GetNearbyStorage)
    (:Is%20Valid
      (Utilities|IsValid _returnvalue_2
        (:Is%20Valid
          (bind _output_get (LocalVariables|SetLocalItemsContainer _returnvalue_2))
          (if (Default|IsWidgetVisible? _output_get) ; We only want to do something if we are watching the widget
            (CallFunction|TransferItem (LocalVariables|GetLocalItemsContainer) -1 (LocalVariables|GetLocalClickedSlot))
            (return)
            (else
              (return))))
        (:Is%20Not%20Valid
          (return))))
    (:Is%20Not%20Valid
      (Utilities|IsValid (Variables|Default|GetNearbySeller)
        (:Is%20Valid
          (Utilities|IsValid _returnvalue
            (:Is%20Valid
              (bind _output_get_2 (LocalVariables|SetLocalItemsContainer _returnvalue))
              (if (Default|IsWidgetVisible? _output_get_2)
                (CallFunction|SellItem (LocalVariables|GetLocalClickedSlot))
                (return)
                (else
                  (return))))
            (:Is%20Not%20Valid
              (return))))
        (:Is%20Not%20Valid
          (return))))))

(fn HandleSlotDrop
  (params (DroppedSlot :type Object%20Object%20Reference) (DroppedIndex :type Integer))
  (LocalVariables|SetLocalDroppedSlot DroppedSlot)
  (LocalVariables|SetLocalDroppedIndex DroppedIndex)
  (bind _aswb_item_container_slot (Utilities|Casting|CastToWB_ItemContainerSlot (LocalVariables|GetLocalDroppedSlot))
    (:then
      (bind _output_get (LocalVariables|SetLocalItemSlot _aswb_item_container_slot))
      (switch Utilities|FlowControl|Switch|Switchone_ContainerType (Variables|/Game/OpenRPG/InventorySystem/Widgets/WB_ItemContainerSlot.WB_ItemContainerSlot_C|GetContainer _output_get)
        (:NewEnumerator0
          (if (Variables|/Game/OpenRPG/InventorySystem/Widgets/WB_ItemsContainerGrid.WB_ItemsContainerGrid_C|GetSplitKeyDown? (Variables|Default|GetContainerGridWidget))
            (bind _success_ (CallFunction|SplitStack (Variables|/Game/OpenRPG/InventorySystem/Widgets/WB_ItemContainerSlot.WB_ItemContainerSlot_C|GetSlotIndex (LocalVariables|GetLocalItemSlot)) (/ (Variables|/Game/OpenRPG/InventorySystem/Widgets/WB_ItemContainerSlot.WB_ItemContainerSlot_C|GetAmount (LocalVariables|GetLocalItemSlot)) (Variables|Default|GetSplitDivideAmount)) (LocalVariables|GetLocalDroppedIndex)))
            (if _success_
              (return)
              (else
                _)))
          (bind _success__2 (CallFunction|AddAmountfromIndextoIndex (Variables|/Game/OpenRPG/InventorySystem/Widgets/WB_ItemContainerSlot.WB_ItemContainerSlot_C|GetSlotIndex (LocalVariables|GetLocalItemSlot)) (LocalVariables|GetLocalDroppedIndex)))
          (if _success__2
            (return)
            (else
              (CallFunction|SwapItems (Variables|/Game/OpenRPG/InventorySystem/Widgets/WB_ItemContainerSlot.WB_ItemContainerSlot_C|GetSlotIndex (LocalVariables|GetLocalItemSlot)) (LocalVariables|GetLocalDroppedIndex))
              (return))))
        (:NewEnumerator1
          (Default|TransferItem (Variables|/Game/OpenRPG/InventorySystem/Widgets/WB_ItemContainerSlot.WB_ItemContainerSlot_C|GetItemsContainerComponent (LocalVariables|GetLocalItemSlot)) self (LocalVariables|GetLocalDroppedIndex) (Variables|/Game/OpenRPG/InventorySystem/Widgets/WB_ItemContainerSlot.WB_ItemContainerSlot_C|GetSlotIndex (LocalVariables|GetLocalItemSlot)))
          (return))
        (:NewEnumerator2
          (Default|BuyItem (.AsBPC%20Seller (Utilities|Casting|CastToBPC_Seller (Variables|/Game/OpenRPG/InventorySystem/Widgets/WB_ItemContainerSlot.WB_ItemContainerSlot_C|GetItemsContainerComponent (LocalVariables|GetLocalItemSlot)))) (Variables|/Game/OpenRPG/InventorySystem/Widgets/WB_ItemContainerSlot.WB_ItemContainerSlot_C|GetSlotIndex (LocalVariables|GetLocalItemSlot)) (LocalVariables|GetLocalDroppedIndex))
          (return))))
    (:CastFailed
      (bind _aswb_equipment_slot (Utilities|Casting|CastToWB_EquipmentSlot (LocalVariables|GetLocalDroppedSlot))) ; Is an equipment slot
      (Default|UnequipItem (Variables|/Game/OpenRPG/EquipmentSystem/Widgets/WB_EquipmentSlot.WB_EquipmentSlot_C|GetEquipmentComponent _aswb_equipment_slot) (Variables|/Game/OpenRPG/EquipmentSystem/Widgets/WB_EquipmentSlot.WB_EquipmentSlot_C|GetType _aswb_equipment_slot) 0 false)
      (return))))