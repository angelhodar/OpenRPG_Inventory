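; Base world pickup actor that gives the player an item and amount through interaction.
; The construction script loads the DT_Items row for ItemID and applies its mesh, scale and interaction radius, so instances preview in the editor.
; The collision sphere registers the pickup as nearby with BPC_InventoryHandler and toggles the interact widget.
; Interacting adds the item to the inventory and destroys the actor only on success.
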(event OnComponentBeginOverlap(Colision)
  (params (OverlappedComponent :type Primitive%20Component%20Object%20Reference) (OtherActor :type Actor%20Object%20Reference) (OtherComp :type Primitive%20Component%20Object%20Reference) (OtherBodyIndex :type Integer) (bFromSweep :type Boolean) (SweepResult :type Hit%20Result%20Structure%20%28by%20ref%29))
  (bind _returnvalue (Actor|GetComponentbyClass OtherActor "/Game/OpenRPG/InventorySystem/Blueprints/BPC_InventoryHandler.BPC_InventoryHandler_C"))
  (Utilities|IsValid _returnvalue
    (:Is%20Valid
      (Default|AddNearbyItem _returnvalue self)
      (Rendering|SetVisibility (Variables|Default|GetInteractWidget) true false) ; Makes the interact widget visible
    )))

(event OnComponentEndOverlap(Colision)
  (params (OverlappedComponent :type Primitive%20Component%20Object%20Reference) (OtherActor :type Actor%20Object%20Reference) (OtherComp :type Primitive%20Component%20Object%20Reference) (OtherBodyIndex :type Integer))
  (bind _returnvalue (Actor|GetComponentbyClass OtherActor "/Game/OpenRPG/InventorySystem/Blueprints/BPC_InventoryHandler.BPC_InventoryHandler_C"))
  (Utilities|IsValid _returnvalue
    (:Is%20Valid
      (Default|RemoveNearbyItem _returnvalue self)
      (Rendering|SetVisibility (Variables|Default|GetInteractWidget) false false) ; Makes the interact widget unvisible
    )))

(event EventBeginPlay
  (|CallParentFunction) ; Here we creates a valid reference to the InteractText widget
  (Default|Initialize (Variables|Default|GetWB_InteractText) (Utilities|Text|FormatText "{Name} x{Amount}" (Utilities|Text|ToText(Name) (Utilities|Struct|Breaks_ItemData (Variables|Default|GetItemData))) (Variables|Default|GetAmount)) "Press [E] to interact!")
  (CallFunction|SetVisualProperties))

(event EventOnInteract
  (params (Player :type BP%20Master%20Character%20Object%20Reference))
  (|CallParentFunction Player) ; This just sets the player controller as a class variable
  (bind _success_ (Default|AddIItem(Public) (Variables|/Game/OpenRPG/InventorySystem/Blueprints/AbstractClasses/BP_MasterCharacter.BP_MasterCharacter_C|GetBPC_InventoryHandler (Variables|Default|GetPlayer)) (Variables|Default|GetItemID) (Variables|Default|GetAmount))) ; We try to add the item
  (if _success_ ; Not enough space?
    (Default|RemoveNearbyItem (Variables|/Game/OpenRPG/InventorySystem/Blueprints/AbstractClasses/BP_MasterCharacter.BP_MasterCharacter_C|GetBPC_InventoryHandler (Variables|Default|GetPlayer)) self)
    (Actor|DestroyActor) ; Destroy self
  ))

(fn ConstructionScript
  (|CallParentFunction)
  (if (!= (Variables|Default|GetItemID) -1)
    (bind _returnvalue (Utilities|GetDataTableRow "/Game/OpenRPG/InventorySystem/Blueprints/Items/DataTables/DT_Items.DT_Items" (Utilities|String|StringToName (Utilities|String|ToString(Integer) (Variables|Default|GetItemID)))) ; Get the info from the data table
      (:then
        (Variables|Default|SetItemData _returnvalue)
        (CallFunction|SetVisualProperties)))))

(fn SetVisualProperties
  (bind _itemdata (Variables|Default|GetItemData))
  (bind _itemdata_2 (Variables|Default|GetItemData))
  (bind (_meshscale _interactradius) (Utilities|Struct|Breaks_ItemData _itemdata))
  (bind _worldmesh (Utilities|Struct|Breaks_ItemData _itemdata_2))
  (Components|StaticMesh|SetStaticMesh (Variables|Default|GetMesh) _worldmesh)
  (Rendering|Material|SetMaterial (Variables|Default|GetMesh) 0 (Rendering|Material|GetMaterial _worldmesh 0))
  (Transformation|SetWorldScale3D (Variables|Default|GetMesh) _meshscale)
  (Components|Sphere|SetSphereRadius (Variables|Default|GetColision) _interactradius false)
  (return))