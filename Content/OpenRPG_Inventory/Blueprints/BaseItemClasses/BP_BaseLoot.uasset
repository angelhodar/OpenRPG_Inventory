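; Base Blueprint for usable loot items in the OpenRPG inventory, which open into other items when used.
; On use it calls the parent handler, then ManageLoot fetches an item list from the item's loot data row name and adds it to the player's inventory component.
; One unit of the loot item is removed from the clicked slot only if the add succeeds; failures print debug messages.
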(event EventOnItemUsed
  (|CallParentFunction) ; Just to keep the debug message :P
  (CallFunction|ManageLoot))

(fn ConstructionScript
  (|CallParentFunction))

(fn ManageLoot
  (bind _itemdata (Variables|Default|GetItemData))
  (bind _lootdatarowname (Utilities|Struct|Breaks_ItemData _itemdata))
  (if (Utilities|Name|NotEqual(Name) _lootdatarowname "None")
    (bind _output_get (LocalVariables|SetLocalLoot (CallFunction|GetItemsListbyRow _lootdatarowname)))
    (if (!= (Utilities|Array|Length _output_get) 0)
      (bind _success_ (Default|AddItems (Variables|Default|GetPlayerInventoryComponent) (LocalVariables|GetLocalLoot)))
      (if _success_
        (Default|RemoveIndexAmount (Variables|Default|GetPlayerInventoryComponent) (Variables|Default|GetClickedSlotIndex) 1)
        (return)
        (else
          (Development|PrintString "Not enough space to open the loot!")
          (return)))
      (else
        (Development|PrintString (Utilities|String|Append "The row " (Utilities|String|ToString(Name) (Utilities|Struct|Breaks_ItemData (Variables|Default|GetItemData))) " doesnt have any items") true true "(R=1.000000,G=0.000000,B=0.012087,A=1.000000)" 1e+01)
        (return)))
    (else
      (Development|PrintString "Invalid loot row name")
      (return))))