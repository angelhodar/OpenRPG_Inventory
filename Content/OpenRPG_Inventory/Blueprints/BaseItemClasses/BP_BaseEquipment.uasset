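; Base item class for equippable items in the OpenRPG inventory, which equips the item when it is used.
; On BeginPlay it runs the parent logic and caches the player's equipment component.
; OnItemUsed calls the parent, kept for its debug message, then has that component equip from the player inventory at the clicked slot index.
; The author marks this event as the place to substitute custom equip logic.
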(event EventBeginPlay
  ;[0.08558 0.3564 1] Set also the equipment component
  (|CallParentFunction)
  (Variables|Default|SetPlayerEquipmentComponent (CallFunction|GetPlayerEquipment)))

(event EventOnItemUsed
  ;[0.1043 1 0.1512] If you have your own way to equip items, it should be implemented here. This is my way of doing it
  (|CallParentFunction) ; Just to keep the debug message :P
  (Default|EquipfromContainer (Variables|Default|GetPlayerEquipmentComponent) (Variables|Default|GetPlayerInventoryComponent) (Variables|Default|GetClickedSlotIndex)))

(fn ConstructionScript
  (|CallParentFunction))