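; BP_BaseConsumable is the inventory system's base consumable item, which is removed from the player's inventory only when its use succeeds.
; UseItem runs the parent logic that triggers OnItemUsed, then removes one from the clicked slot if UsedSuccessfully is set and resets the flag.
; OnItemUsed sets that flag at the end of its logic, so an item with no effect, like a potion at full health, can be kept.
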(event EventOnItemUsed
  ;[0.069 0.2313 1] Here the logic is the same but make sure you set this boolean at the end of the execution
  (|CallParentFunction) ; Just to keep the debug message :P
  (Variables|Default|SetUsedSuccessfully? true))

(event EventUseItem
  (params (Clicked%20Slot%20Index :type Integer))
  ;[0.1043 1 0.1512] Here the idea is the same, but to avoid some bugs like for example you use a potion but your health is already 100% the only thing you need to do is setting the boolean UsedSuccessfully? at the end of your OnItemUsed logic, that way the inventory will only remove that potion if it was used
  (Utilities|FlowControl|Sequence
    (:then_0
      (|CallParentFunction Clicked%20Slot%20Index) ; First we execute the overriden item logic, which will call OnItemUsed
    )
    (:then_1
      (if (Variables|Default|GetUsedSuccessfully?)
        (Default|RemoveIndexAmount (Variables|Default|GetPlayerInventoryComponent) (Variables|Default|GetClickedSlotIndex) 1)
        (Variables|Default|SetUsedSuccessfully? false) ; Reset for next use
      ))))

(fn ConstructionScript
  (|CallParentFunction))