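; InventorySave is a save data Blueprint for the OpenRPG inventory system that stores container contents and player inventory data.
; Two maps, SavedContainers and SavedPlayerData, hold entries keyed by a save name.
; Save events add an entry to the matching map, and load functions look up a name and return a found flag with the stored data.
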(event EventSaveContainer
  (params (SaveName :type String) (Data :type S%20Container%20Save%20Data%20Structure))
  (Utilities|Map|Add (Variables|Default|GetSavedContainers) SaveName Data))

(event EventSavePlayerInventoryData
  (params (SaveName :type String) (Data :type S%20Player%20Inventory%20Save%20Data%20Structure))
  (Utilities|Map|Add (Variables|Default|GetSavedPlayerData) SaveName Data))

(fn LoadContainer
  (params (SaveName :type String))
  (bind _savedcontainers (Variables|Default|GetSavedContainers))
  (bind (_value _returnvalue) (Utilities|Map|Find _savedcontainers SaveName))
  (return _returnvalue _value))

(fn LoadPlayerInventoryData
  (params (SaveName :type String))
  (bind _savedplayerdata (Variables|Default|GetSavedPlayerData))
  (bind (_value _returnvalue) (Utilities|Map|Find _savedplayerdata SaveName))
  (return _returnvalue _value))