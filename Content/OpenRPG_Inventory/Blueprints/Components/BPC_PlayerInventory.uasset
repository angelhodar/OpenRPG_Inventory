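; Player inventory component that handles item use, money, selling and interaction with nearby items, storages and shops.
; Slot clicks use items through spawned item actors cached per item, or quick-transfer or sell them while the quick-action key is held.
; Slot drops route by source to rearranging, storage transfer, shop purchase or unequipping.
; BeginPlay polls until its grid widget is valid, and money persists through the save/load extra-data events.
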(event Custom|OpenStorage
  ;[0.1548 1 0.02316] Input events from player to use with interactables
  (Utilities|IsValid (Variables|Interactables|GetNearbyStorage)
    (:Is%20Valid
      (Class|BPIWorldInteraction|OnInteract(Message) (Variables|Interactables|GetNearbyStorage) (Components|GetOwner)))))

(event Custom|OpenShop
  ;[0.1548 1 0.02316] Input events from player to use with interactables
  (Utilities|IsValid (Variables|Interactables|GetNearbySeller)
    (:Is%20Valid
      (Class|BPIWorldInteraction|OnInteract(Message) (Variables|Interactables|GetNearbySeller) (Components|GetOwner)))))

(event Custom|PickUpItem
  (bind _nearbyitems (Variables|Interactables|GetNearbyItems))
  (bind _output (Utilities|Array|Get(acopy) _nearbyitems))
  ;[0.1548 1 0.02316] Input events from player to use with interactables
  (Utilities|IsValid _output
    (:Is%20Valid
      (Class|BPIWorldInteraction|OnInteract(Message) _output (Components|GetOwner)))))

(event EventOnSlotDrop
  (params (DroppedSlot :type Object%20Object%20Reference) (DroppedIndex :type Integer))
  ;[0.02391 0.00239 1] Override slot drop
  (CallFunction|HandleSlotDrop DroppedSlot DroppedIndex))

(event EventBeginPlay
  ;[0.03063 0.5441 1] BeginPlay
  (|CallParentFunction)
  (Utilities|IsValid (Variables|Default|GetContainerGridWidget) :!label _label
    (:Is%20Valid
      (CallFunction|UpdateContainerWidget))
    (:Is%20Not%20Valid
      (Utilities|FlowControl|Delay 0.1)
      (bind _widget (Class|BPIContainerWidgets|GetContainerWidget(Message) (CallFunction|GetContainerWidgetsOwner) (Variables|Default|GetContainerType)))
      (Variables|Default|SetContainerGridWidget _widget)
      (goto _label))))

(event EventOnSaveExtraData
  (params (SaveName :type String) (SaveObject :type Object%20Object%20Reference))
  ;[1 0.7938 0.03439] Override of the save/load extra data events to manage the SavedMoney variable in ItemsSave class
  (Class|BPIPlayerInventorySave|SavePlayerInventoryData(Message) SaveObject SaveName (CallFunction|CreateSaveData)))

(event EventOnLoadExtraData
  (params (SaveName :type String) (SaveObject :type Object%20Object%20Reference))
  ;[1 0.7938 0.03439] Override of the save/load extra data events to manage the SavedMoney variable in ItemsSave class
  (bind (_found_ _data) (Class|BPIPlayerInventorySave|LoadPlayerInventoryData(Message) SaveObject SaveName))
  (if _found_
    (CallFunction|AddMoney (Utilities|Struct|Breaks_PlayerInventorySaveData _data))))

(event EventOnSlotClicked
  (params (ClickedIndex :type Integer))
  ;[1 0.03646 0.1158] Overriden event to use an item when a ui slot is clicked
  (if (Game|Player|IsInputKeyDown (Game|GetPlayerController 0) (Variables|PlayerSettings|GetQuickActionKey))
    (CallFunction|HandleQuickAction ClickedIndex)
    (else
      (CallFunction|UseItem ClickedIndex))))

(fn CanUseItem?
  (params (Index :type Integer))
  (LocalVariables|SetLocalIndex Index)
  (LocalVariables|SetLocalPlayerLevel (CallFunction|GetPlayerLevel))
  (return (Math|Boolean|ANDBoolean (not (CallFunction|IsSlotEmpty? (LocalVariables|GetLocalIndex))) (.Usable? (Utilities|Struct|Breaks_ItemData (CallFunction|GetItemDatabyRow (Utilities|Struct|Breaks_InventoryItem (CallFunction|GetItematIndex (LocalVariables|GetLocalIndex)))))) (>= (LocalVariables|GetLocalPlayerLevel) (.FromLvl (Utilities|Struct|Breaks_ItemData (CallFunction|GetItemDatabyRow (Utilities|Struct|Breaks_InventoryItem (CallFunction|GetItematIndex (LocalVariables|GetLocalIndex))))))))))

(fn AddNearbyItem
  (params (NearbyActor :type BP%20World%20Item%20Object%20Reference))
  (Utilities|Array|AddUnique (Variables|Interactables|GetNearbyItems) NearbyActor)
  (return))

(fn RemoveNearbyItem
  (params (NearbyActor :type BP%20World%20Item%20Object%20Reference))
  (Utilities|Array|RemoveItem (Variables|Interactables|GetNearbyItems) NearbyActor)
  (return))

(fn AddMoney
  (params (Amount :type Integer))
  (bind _output_get (LocalVariables|SetLocalAmount Amount))
  (bind _output_get_2 (LocalVariables|SetLocalNewAmount (+ _output_get (Variables|Default|GetCurrentMoney))))
  (if (and (<= _output_get_2 (Variables|PlayerSettings|GetMaxMoney)) (>= (LocalVariables|GetLocalNewAmount) 0)) ; Are we not going to have more than the max money or below 0?
    (Variables|Default|SetCurrentMoney (LocalVariables|GetLocalNewAmount))
    (Default|CallOnMoneyAmountChanged (LocalVariables|GetLocalAmount) (LocalVariables|GetLocalNewAmount))
    (return true)
    (else
      (return false))))

(fn SellItem
  (params (Index :type Integer))
  (LocalVariables|SetLocalIndex Index)
  (if (not (CallFunction|IsSlotEmpty? (LocalVariables|GetLocalIndex)))
    (LocalVariables|SetLocalItem (.Item (Utilities|Struct|Breaks_InventoryItem (CallFunction|GetItematIndex (LocalVariables|GetLocalIndex)))))
    (LocalVariables|SetLocalAmount (.Amount (Utilities|Struct|Breaks_InventoryItem (CallFunction|GetItematIndex (LocalVariables|GetLocalIndex)))))
    (if (Utilities|Enum|NotEqual(Enum) (.Type (Utilities|Struct|Breaks_ItemData (CallFunction|GetItemDatabyRow (LocalVariables|GetLocalItem)))) "NewEnumerator2")
      (bind _output_get (LocalVariables|SetLocalBenefit (* (.Value (Utilities|Struct|Breaks_ItemData (CallFunction|GetItemDatabyRow (LocalVariables|GetLocalItem)))) (LocalVariables|GetLocalAmount))))
      (bind _success_ (CallFunction|AddMoney _output_get))
      (if _success_
        (CallFunction|RemoveIndexAmount (LocalVariables|GetLocalIndex) (LocalVariables|GetLocalAmount))
        (return true)
        (else
          (return false)))
      (else
        (return false)))
    (else
      (return false))))

(fn UseItem
  (params (Index :type Integer))
  (bind _output_get (LocalVariables|SetLocalIndex Index))
  (if (CallFunction|CanUseItem? _output_get)
    (bind _output_get_2 (LocalVariables|SetLocalItem (Utilities|Struct|Breaks_InventoryItem (CallFunction|GetItematIndex (LocalVariables|GetLocalIndex)))))
    (bind _output_get_3 (LocalVariables|SetLocalItemData (CallFunction|GetItemDatabyRow _output_get_2)))
    (if (Utilities|IsValidClass (Utilities|Struct|Breaks_ItemData _output_get_3))
      (bind _output_get_4 (LocalVariables|SetLocalItemToUse (CallFunction|GetSpawnedItem (LocalVariables|GetLocalItem))))
      (Utilities|IsValid _output_get_4
        (:Is%20Valid
          _)
        (:Is%20Not%20Valid
          (bind _returnvalue (Game|SpawnActorfromClass (Utilities|Struct|Breaks_ItemData (LocalVariables|GetLocalItemData)) (Math|Transform|MakeTransform "0, 0, 0" "0, 0, 0" "1,1,1") "AlwaysSpawn" 0 (LocalVariables|GetLocalItem) (LocalVariables|GetLocalItemData) self 0)) ; This will spawn the class associated with the item that contains all the logic that has to be excuted
          (bind _output_get_5 (LocalVariables|SetLocalItemToUse _returnvalue))
          (CallFunction|AddSpawnedActor (LocalVariables|GetLocalItem) _output_get_5)))
      (Default|UseItem (LocalVariables|GetLocalItemToUse) (LocalVariables|GetLocalIndex)) ; Starts the item logic execution based on its type
      (Default|CallOnItemUsed (LocalVariables|GetLocalItem))
      (return true)
      (else
        (Default|CallOnItemUsed (LocalVariables|GetLocalItem))
        (return true)))
    (else
      (return false))))

(fn HandleQuickAction
  (params (ClickedIndex :type Integer))
  (bind _nearbystorage (Variables|Interactables|GetNearbyStorage))
  (bind _nearbyseller (Variables|Interactables|GetNearbySeller))
  (bind _returnvalue (Actor|GetComponentbyClass _nearbyseller "/Game/OpenRPG_Inventory/Blueprints/Components/BPC_ItemsContainer.BPC_ItemsContainer_C"))
  (bind _returnvalue_2 (Actor|GetComponentbyClass _nearbystorage "/Game/OpenRPG_Inventory/Blueprints/Components/BPC_ItemsContainer.BPC_ItemsContainer_C"))
  (LocalVariables|SetLocalClickedSlot ClickedIndex)
  (Utilities|IsValid (Variables|Interactables|GetNearbyStorage)
    (:Is%20Valid
      (Utilities|IsValid _returnvalue_2
        (:Is%20Valid
          (LocalVariables|SetLocalItemsContainer _returnvalue_2)
          (bind _widget (Class|BPIContainerWidgets|GetContainerWidget(Message) (CallFunction|GetContainerWidgetsOwner) (Variables|Default|GetContainerType)))
          (if (Widget|IsVisible _widget) ; We only want to do something if we are watching the widget
            (CallFunction|TransferItem (LocalVariables|GetLocalItemsContainer) -1 (LocalVariables|GetLocalClickedSlot))
            (return)
            (else
              (return))))
        (:Is%20Not%20Valid
          (return))))
    (:Is%20Not%20Valid
      (Utilities|IsValid (Variables|Interactables|GetNearbySeller)
        (:Is%20Valid
          (Utilities|IsValid _returnvalue
            (:Is%20Valid
              (LocalVariables|SetLocalItemsContainer _returnvalue)
              (bind _widget_2 (Class|BPIContainerWidgets|GetContainerWidget(Message) (CallFunction|GetContainerWidgetsOwner) (Variables|Default|GetContainerType)))
              (if (Widget|IsVisible _widget_2)
                (CallFunction|SellItem (LocalVariables|GetLocalClickedSlot))
                (return)
                (else
                  (return))))
            (:Is%20Not%20Valid
              (return))))
        (:Is%20Not%20Valid
          (return))))))

(fn HandleSlotDrop
  (params (DroppedSlot :type Object%20Object%20Reference) (DroppedIndex :type Integer))
  (LocalVariables|SetLocalDroppedSlot DroppedSlot)
  (LocalVariables|SetLocalDroppedIndex DroppedIndex)
  (bind _aswb_item_container_slot (Utilities|Casting|CastToWB_ItemContainerSlot (LocalVariables|GetLocalDroppedSlot))
    (:then
      (bind _output_get (LocalVariables|SetLocalItemSlot _aswb_item_container_slot))
      (switch Utilities|FlowControl|Switch|Switchone_ContainerType (Variables|/Game/OpenRPG_Inventory/Widgets/WB_ItemContainerSlot.WB_ItemContainerSlot_C|GetContainer _output_get)
        (:NewEnumerator0
          (CallFunction|HandleSelfContainerSlotDrop (LocalVariables|GetLocalDroppedSlot) (LocalVariables|GetLocalDroppedIndex))
          (return))
        (:NewEnumerator1
          (Default|TransferItem (Variables|/Game/OpenRPG_Inventory/Widgets/WB_ItemContainerSlot.WB_ItemContainerSlot_C|GetItemsContainerComponent (LocalVariables|GetLocalItemSlot)) self (LocalVariables|GetLocalDroppedIndex) (Variables|/Game/OpenRPG_Inventory/Widgets/WB_ItemContainerSlot.WB_ItemContainerSlot_C|GetSlotIndex (LocalVariables|GetLocalItemSlot)))
          (return))
        (:NewEnumerator2
          (Default|BuyItem (.AsBPC%20Shop (Utilities|Casting|CastToBPC_Shop (Variables|/Game/OpenRPG_Inventory/Widgets/WB_ItemContainerSlot.WB_ItemContainerSlot_C|GetItemsContainerComponent (LocalVariables|GetLocalItemSlot)))) (Variables|/Game/OpenRPG_Inventory/Widgets/WB_ItemContainerSlot.WB_ItemContainerSlot_C|GetSlotIndex (LocalVariables|GetLocalItemSlot)) (LocalVariables|GetLocalDroppedIndex))
          (return))))
    (:CastFailed
      (bind _aswb_equipment_slot (Utilities|Casting|CastToWB_EquipmentSlot (LocalVariables|GetLocalDroppedSlot))) ; Is an equipment slot
      (Default|UnequipItem (Variables|/Game/OpenRPG_Equipment/Widgets/WB_EquipmentSlot.WB_EquipmentSlot_C|GetEquipmentComponent _aswb_equipment_slot) (Variables|/Game/OpenRPG_Equipment/Widgets/WB_EquipmentSlot.WB_EquipmentSlot_C|GetType _aswb_equipment_slot) (LocalVariables|GetLocalDroppedIndex) false)
      (return))))

(fn GetSpawnedItem
  (params (Item :type Name))
  (return (.Value (Utilities|Map|Find (Variables|Default|GetSpawnedItems) Item))))

(fn AddSpawnedActor
  (params (Item :type Name) (Actor :type BP%20Base%20Item%20Object%20Reference))
  (Utilities|Map|Add (Variables|Default|GetSpawnedItems) Item Actor)
  (return))

(fn CreateSaveData
  (return (Utilities|Struct|Makes_PlayerInventorySaveData (Variables|Default|GetCurrentMoney))))