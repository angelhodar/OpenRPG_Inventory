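; BPC_Storage is the inventory component for storage containers, handling item movement between storage and the player inventory.
; It overrides the slot events: clicking a slot transfers that item to the player inventory.
; Drops go to HandleSlotDrop, which branches on the source slot's container type.
; Player items transfer into the dropped index, storage items use the self-container drop handler, and shop or non-item slots are ignored.
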(event EventOnSlotClicked
  (params (ClickedIndex :type Integer))
  ;[1 0.03646 0.1158] Override On Slot Clicked: In this case it just transfers the clicked index to the player inventory...
  (CallFunction|TransferItem (CallFunction|GetPlayerInventory) -1 ClickedIndex))

(event EventOnSlotDrop
  (params (DroppedSlot :type Object%20Object%20Reference) (DroppedIndex :type Integer))
  ;[0.02391 0.00239 1] Override On Slot Drop: Calls HandleSlotDrop to keep code clean
  (CallFunction|HandleSlotDrop DroppedSlot DroppedIndex))

(fn HandleSlotDrop
  (params (DroppedSlot :type Object%20Object%20Reference) (DroppedIndex :type Integer))
  (LocalVariables|SetLocalDroppedSlot DroppedSlot)
  (LocalVariables|SetLocalDroppedIndex DroppedIndex)
  (bind _aswb_item_container_slot (Utilities|Casting|CastToWB_ItemContainerSlot (LocalVariables|GetLocalDroppedSlot))
    (:then
      (bind _output_get (LocalVariables|SetLocalItemSlot _aswb_item_container_slot))
      (switch Utilities|FlowControl|Switch|Switchone_ContainerType (Variables|/Game/OpenRPG_Inventory/Widgets/WB_ItemContainerSlot.WB_ItemContainerSlot_C|GetContainer _output_get)
        (:NewEnumerator0
          (Default|TransferItem (CallFunction|GetPlayerInventory) self (LocalVariables|GetLocalDroppedIndex) (Variables|/Game/OpenRPG_Inventory/Widgets/WB_ItemContainerSlot.WB_ItemContainerSlot_C|GetSlotIndex (LocalVariables|GetLocalItemSlot)))
          (return))
        (:NewEnumerator1
          (CallFunction|HandleSelfContainerSlotDrop (LocalVariables|GetLocalDroppedSlot) (LocalVariables|GetLocalDroppedIndex))
          (return))
        (:NewEnumerator2
          (return))))
    (:CastFailed
      (return))))