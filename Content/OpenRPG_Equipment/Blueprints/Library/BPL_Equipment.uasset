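; BPL_Equipment is a Blueprint function library of shared lookups for the OpenRPG equipment system.
; It fetches the first player character's equipment component and player controller (as equipment widget owner), and reads equipment rows from DT_Equipment by name.
; It also supplies a fixed save slot name, which the save getter uses to load the existing EquipmentSave or create a new, unsaved one when none exists.
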(fn GetPlayerEquipment
  (return (Actor|GetComponentbyClass (Game|GetPlayerCharacter (LocalVariables|Get__WorldContext)) "/Game/OpenRPG_Equipment/Blueprints/Components/BPC_Equipment.BPC_Equipment_C")))

(fn GetEquipmentDatabyRow
  (params (Row :type Name))
  (bind _returnvalue (Utilities|GetDataTableRow "/Game/OpenRPG_Equipment/Datatables/DT_Equipment.DT_Equipment" Row)
    (:then
      (return _returnvalue))
    (:RowNotFound
      (return ""))))

(fn GetEquipmentSaveObject
  (bind _output_get (LocalVariables|SetLocalSlotName (Save/Load|GetEquipmentSaveSlotName (LocalVariables|Get__WorldContext))))
  (bind _returnvalue (SaveGame|DoesSaveGameExist _output_get))
  (if _returnvalue
    (bind _returnvalue_2 (SaveGame|LoadGamefromSlot (LocalVariables|GetLocalSlotName)))
    (bind _asequipment_save (Utilities|Casting|CastToEquipmentSave _returnvalue_2)
      (:then
        (return _asequipment_save))
      (:CastFailed
        (return 0)))
    (else
      (bind _returnvalue_3 (SaveGame|CreateSaveGameObject "/Game/OpenRPG_Equipment/Blueprints/Saving/EquipmentSave.EquipmentSave_C"))
      (return _returnvalue_3))))

(fn GetEquipmentWidgetsOwner
  (return (Game|GetPlayerController (LocalVariables|Get__WorldContext))))

(fn GetEquipmentSaveSlotName
  (return "OpenRPG_Equipment"))