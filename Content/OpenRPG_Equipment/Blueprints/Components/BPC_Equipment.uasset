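; Actor component that manages a player's equipped items per slot type, linking BPC_PlayerInventory to the owner through BPI_Equipment.
; Equip and unequip move items to and from inventory, swapping occupied slots or dropping, and update the equipment widget.
; Gear meshes follow the player mesh via master pose, or attach to a custom bone with a relative transform.
; Equipment saves and loads through the game instance or a save slot, re-equipping and respawning item actors on load.
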(event Custom|Initialize
  (bind _returnvalue (Components|GetOwner))
  (bind _returnvalue_2 (Actor|GetComponentbyClass _returnvalue "/Game/OpenRPG_Inventory/Blueprints/Components/BPC_PlayerInventory.BPC_PlayerInventory_C"))
  (if (Utilities|DoesObjectImplementInterface (Components|GetOwner) "/Game/OpenRPG_Equipment/Blueprints/Interfaces/BPI_Equipment.BPI_Equipment_C")
    (if (Variables|Internal|GetHasLoadBeenSuccessful?)
      _
      (else
        (Others|SetupEquipment)))
    (Utilities|IsValid (Variables|Default|GetPlayerInventoryReference)
      (:Is%20Valid
        (bind _widget (Class|BPIEquipmentWidgets|GetEquipmentContainerWidget(Message) (CallFunction|GetEquipmentWidgetsOwner) :!label _label))
        (bind _output_get (Variables|UI|SetEquipmentSlotsContainerWidget _widget))
        (Utilities|IsValid _output_get
          (:Is%20Valid
            (Default|Initialize (Variables|UI|GetEquipmentSlotsContainerWidget) self)
            (Utilities|PrintDebug "Equipment: Initialized successfully!" "(R=0.082484,G=1.000000,B=0.000000,A=1.000000)" 3.0))
          (:Is%20Not%20Valid
            (Utilities|FlowControl|Delay 0.1)
            (goto _label))))
      (:Is%20Not%20Valid
        (Utilities|IsValid _returnvalue_2
          (:Is%20Valid
            (Variables|Default|SetPlayerInventoryReference _returnvalue_2)
            (goto _label))
          (:Is%20Not%20Valid
            (Utilities|PrintDebug "Equipment Your player doesnt have the PlayerInventory component" "(R=0.994792,G=0.070239,B=0.000000,A=1.000000)" 5.0)))))
    (else
      (Utilities|PrintDebug "Equipment Your player doesnt implement the BPL_Equipment interface" "(R=0.994792,G=0.070239,B=0.000000,A=1.000000)" 5.0))))

(event Custom|UpdateEquipmentSlot
  (params (Slot :type e_EquipmentType%20Enum :default "NewEnumerator0"))
  (bind _equipmentslotscontainerwidget (Variables|UI|GetEquipmentSlotsContainerWidget))
  (Utilities|IsValid _equipmentslotscontainerwidget
    (:Is%20Valid
      (Default|UpdateSlot _equipmentslotscontainerwidget Slot))))

(fn GetIteminSlot
  (params (SlotType :type e_EquipmentType%20Enum :default "NewEnumerator0"))
  (return (.Value (Utilities|Map|Find (Variables|General|GetEquipment) SlotType))))

(fn EquipItem
  (params (Item :type Name) (FromInventorySlot :type Integer))
  ;[0.08879 0.8399 1] This part of the code just extracts the necessary data and set it, giving warnings when something is not correctly set.
  (LocalVariables|SetLocalItem Item)
  (LocalVariables|SetLocalClickedInventorySlot FromInventorySlot)
  (Utilities|IsValid (Variables|Default|GetPlayerInventoryReference)
    (:Is%20Valid
      (bind _mesh (Class|BPIEquipment|GetPlayerMesh(Message) (Components|GetOwner)))
      (bind _output_get (LocalVariables|SetLocalPlayerMesh _mesh))
      (Utilities|IsValid _output_get
        (:Is%20Valid
          (bind _output_get_2 (LocalVariables|SetLocalItemData (CallFunction|GetItemDatabyRow (LocalVariables|GetLocalItem))))
          (bind _returnvalue (Class|DataTableFunctionLibrary|DoesDataTableRowExist "/Game/OpenRPG_Equipment/Datatables/DT_Equipment.DT_Equipment" (Utilities|Struct|Breaks_ItemData _output_get_2)))
          (if _returnvalue
            (bind _output_get_3 (LocalVariables|SetLocalEquipmentData (CallFunction|GetEquipmentDatabyRow (Utilities|Struct|Breaks_ItemData _output_get_2))))
            (LocalVariables|SetLocalSlotType (Utilities|Struct|Breaks_EquipmentData _output_get_3))
            (bind _meshcomponent (Class|BPIEquipment|GetEquipmentMeshComponentbyType(Message) (Components|GetOwner) (LocalVariables|GetLocalSlotType)))
            (bind _output_get_4 (LocalVariables|SetLocalMeshComponent _meshcomponent)) ; We get the mesh component of the player that we are going to update
            (Utilities|IsValid _output_get_4
              (:Is%20Valid
                (bind _output_get_5 (LocalVariables|SetLocalEquippedItem (Others|GetIteminSlot (LocalVariables|GetLocalSlotType))))
                (if (Utilities|Name|Equal(Name) _output_get_5 "None") ; Is the slot empty?
                  _
                  (else
                    ;[1 0.09375 0.09375] This part unequips the item already equiped in the slot, and removes the clicked inventory slot
                    (Default|RemoveIndexAmount (Variables|Default|GetPlayerInventoryReference) (LocalVariables|GetLocalClickedInventorySlot) 1) ; First we clean the slot of the item that we are going to equip (we have it stored in the LocalItem variable)
                    (Managment|UnequipItem (LocalVariables|GetLocalSlotType) (LocalVariables|GetLocalClickedInventorySlot) false)
                    (LocalVariables|SetLocalSwap? true)))
                ;[1 0.91 0.07485] This part is responsible of the visual equipment, it updates the player pawn with the skeletal mesh of the item that we are going to equip
                (Utilities|IsValid (Utilities|Struct|Breaks_EquipmentData (LocalVariables|GetLocalEquipmentData)) ; If the mesh isnt valid we skip the visual logic part
                  (:Is%20Valid
                    (Class|SkinnedMeshComponent|SetSkeletalMesh (LocalVariables|GetLocalMeshComponent) (Utilities|Struct|Breaks_EquipmentData (LocalVariables|GetLocalEquipmentData)) true) ; We set the mesh of that component to the one in the equipment data
                    (if (Utilities|Name|Equal(Name) (Utilities|Struct|Breaks_EquipmentData (LocalVariables|GetLocalEquipmentData)) "None") ; If we want to attach the component in a particular bone with custom transform this will have a valid value (only recommended for weapons)
                      (Class|SkinnedMeshComponent|SetMasterPoseComponent (LocalVariables|GetLocalMeshComponent) (LocalVariables|GetLocalPlayerMesh) false) ; If the skeletal mesh has the same skeleton as our player, this function will make it to fit it
                      (else
                        (Transformation|AttachComponentToComponent (LocalVariables|GetLocalMeshComponent) (LocalVariables|GetLocalPlayerMesh) (Utilities|Struct|Breaks_EquipmentData (LocalVariables|GetLocalEquipmentData)) "KeepRelative" "KeepRelative" "KeepRelative" true)
                        (Transformation|SetRelativeTransform (LocalVariables|GetLocalMeshComponent) (Utilities|Struct|Breaks_EquipmentData (LocalVariables|GetLocalEquipmentData)) false false))))
                  (:Is%20Not%20Valid
                    _))
                (Utilities|Map|Add (Variables|General|GetEquipment) (LocalVariables|GetLocalSlotType) (LocalVariables|GetLocalItem))
                (CallFunction|UpdateEquipmentSlot (LocalVariables|GetLocalSlotType))
                (if (or (LocalVariables|GetLocalSwap?) (== (LocalVariables|GetLocalClickedInventorySlot) -1))
                  _
                  (else
                    (Default|RemoveIndexAmount (Variables|Default|GetPlayerInventoryReference) (LocalVariables|GetLocalClickedInventorySlot) 1) ; So we remove the item in that slot, if not we would see it in the equipment slot and in the inventory
                  ))
                (Default|CallOnItemEquipped (LocalVariables|GetLocalItem) (LocalVariables|GetLocalSlotType))
                (return))
              (:Is%20Not%20Valid
                (Utilities|PrintDebug "Equipment: Item equipping aborted, the interface function GetEquipmentMeshComponentByType isnt returning a valid mesh component. Make sure you have implemented it!" "(R=0.869792,G=0.031711,B=0.031711,A=1.000000)" 1e+01)
                (return)))
            (else
              (Utilities|PrintDebug (Utilities|String|Append "Equipment: Item equipping aborted, the equipment data row for item " (Utilities|String|ToString(Name) (LocalVariables|GetLocalItem)) " doesnt exist in DT_Equipment datatable") "(R=0.869792,G=0.031711,B=0.031711,A=1.000000)" 8.0)
              (return))))
        (:Is%20Not%20Valid
          (Utilities|PrintDebug "Equipment: Item equipping aborted, the interface function GetPlayerMesh isnt returning a valid mesh component. Make sure you have implemented it!" "(R=0.869792,G=0.031711,B=0.031711,A=1.000000)" 1e+01)
          (return))))
    (:Is%20Not%20Valid
      (Utilities|PrintDebug "Equipment: Item equipping aborted, the player inventory is not valid!" "(R=0.869792,G=0.031711,B=0.031711,A=1.000000)" 6.0)
      (return))))

(fn UnequipItem
  (params (SlotType :type e_EquipmentType%20Enum :default "NewEnumerator0") (ToSpecificInventoryIndex :type Integer) (Drop? :type Boolean))
  (LocalVariables|SetLocalSlotType SlotType)
  (LocalVariables|SetLocalSpecificIndex ToSpecificInventoryIndex)
  (LocalVariables|SetLocalDrop Drop?)
  (Utilities|IsValid (Variables|Default|GetPlayerInventoryReference)
    (:Is%20Valid
      (bind _meshcomponent (Class|BPIEquipment|GetEquipmentMeshComponentbyType(Message) (Components|GetOwner) (LocalVariables|GetLocalSlotType)))
      (bind _output_get (LocalVariables|SetLocalMeshComponent _meshcomponent)) ; We get the mesh component of the player that we are going to update
      (Utilities|IsValid _output_get
        (:Is%20Valid
          (LocalVariables|SetLocalEquippedItem (Others|GetIteminSlot (LocalVariables|GetLocalSlotType)))
          (if (LocalVariables|GetLocalDrop)
            (Default|DropItem (Variables|Default|GetPlayerInventoryReference) (Utilities|Struct|Makes_InventoryItem (LocalVariables|GetLocalEquippedItem) 1))
            (elif (!= (LocalVariables|GetLocalSpecificIndex) -1) ; If true it means we have to unequip to a specifil inventory index (we are dragging from the equipment slot to an inventory slot)
              (if (Default|IsSlotEmpty? (Variables|Default|GetPlayerInventoryReference) (LocalVariables|GetLocalSpecificIndex)) ; If the slot is empty it means we can drop the item in the inventory slot
                (Default|AddItemtoIndex (Variables|Default|GetPlayerInventoryReference) (Utilities|Struct|Makes_InventoryItem (LocalVariables|GetLocalEquippedItem) 1) (LocalVariables|GetLocalSpecificIndex)) ; We add it
                (else
                  (Utilities|PrintDebug "Equipment: Item unequipping aborted, trying to unequip to a not empty slot" "(R=0.869792,G=0.031711,B=0.031711,A=1.000000)" 6.0)
                  (return false)))
              (else
                (bind _success_ (Default|AddIItem (Variables|Default|GetPlayerInventoryReference) (Utilities|Struct|Makes_InventoryItem (LocalVariables|GetLocalEquippedItem) 1))) ; We unequip in the first empty slot
                (if _success_
                  _
                  (else
                    (Utilities|PrintDebug "Equipment: Item unequipping aborted, AddItem function failed, maybe not enough space in inventory" "(R=0.869792,G=0.031711,B=0.031711,A=1.000000)" 6.0)
                    (return false))))))
          (Class|SkinnedMeshComponent|SetSkeletalMesh (LocalVariables|GetLocalMeshComponent) 0 true) ; Resets the visual equipment, it simulates that we unequipped the item
          (Utilities|Map|Add (Variables|General|GetEquipment) (LocalVariables|GetLocalSlotType) (LocalVariables|GetLocalNone))
          (CallFunction|UpdateEquipmentSlot (LocalVariables|GetLocalSlotType))
          (Default|CallOnItemUnequipped (LocalVariables|GetLocalEquippedItem) (LocalVariables|GetLocalSlotType) (LocalVariables|GetLocalDrop))
          (return true))
        (:Is%20Not%20Valid
          (Utilities|PrintDebug "Equipment: Item unequipping aborted, the interface function GetEquipmentMeshComponentByType isnt returning a valid mesh component. Make sure you have implemented it!" "(R=0.869792,G=0.031711,B=0.031711,A=1.000000)" 1e+01)
          (return false))))
    (:Is%20Not%20Valid
      (Utilities|PrintDebug "Equipment: Item unequipping aborted, the player inventory is not valid!" "(R=0.869792,G=0.031711,B=0.031711,A=1.000000)" 6.0)
      (return false))))

(fn SaveEquipment
  (params (SaveName :type String) (ToGameInstance? :type Boolean))
  (LocalVariables|SetLocalSaveName SaveName)
  (bind _output_get (LocalVariables|SetLocalToGameInstance ToGameInstance?))
  (if _output_get
    (if (Utilities|DoesObjectImplementInterface (Game|GetGameInstance) "/Game/OpenRPG_Equipment/Blueprints/Interfaces/BPI_EquipmentSave.BPI_EquipmentSave_C")
      (Class|BPIEquipmentSave|SaveEquipment(Message) (Game|GetGameInstance) (LocalVariables|GetLocalSaveName) (Save/Load|CreateEquipmentSaveData))
      (return)
      (else
        (Utilities|PrintDebug "Equipment: Saving aborted, game instance doesnt implement equipment save interface" "(R=0.968750,G=0.035319,B=0.035319,A=1.000000)" 6.0)
        (return)))
    (else
      (bind _output_get_2 (LocalVariables|SetLocalSaveObject (CallFunction|GetEquipmentSaveObject)))
      (Utilities|IsValid _output_get_2
        (:Is%20Valid
          (if (Utilities|DoesObjectImplementInterface (LocalVariables|GetLocalSaveObject) "/Game/OpenRPG_Equipment/Blueprints/Interfaces/BPI_EquipmentSave.BPI_EquipmentSave_C")
            (Class|BPIEquipmentSave|SaveEquipment(Message) (LocalVariables|GetLocalSaveObject) (LocalVariables|GetLocalSaveName) (Save/Load|CreateEquipmentSaveData))
            (SaveGame|SaveGametoSlot (LocalVariables|GetLocalSaveObject) (CallFunction|GetEquipmentSaveSlotName))
            (return)
            (else
              (Utilities|PrintDebug "Equipment: Saving aborted, save object doesnt implement equipment save interface" "(R=0.968750,G=0.035319,B=0.035319,A=1.000000)" 6.0)
              (return))))
        (:Is%20Not%20Valid
          (Utilities|PrintDebug "Equipment: Saving aborted, GetEquipmentSaveObject has returned a not valid object reference" "(R=0.968750,G=0.035319,B=0.035319,A=1.000000)" 6.0)
          (return))))))

(fn LoadEquipment
  (params (SaveName :type String) (FromGameInstance? :type Boolean))
  (bind _returnvalue (Components|GetOwner))
  (bind _returnvalue_2 (Actor|GetComponentbyClass _returnvalue "/Game/OpenRPG_Inventory/Blueprints/Components/BPC_PlayerInventory.BPC_PlayerInventory_C"))
  (LocalVariables|SetLocalSaveName SaveName)
  (bind _output_get (LocalVariables|SetLocalFromGameInstance? FromGameInstance?))
  (if _output_get
    (if (Utilities|DoesObjectImplementInterface (Game|GetGameInstance) "/Game/OpenRPG_Equipment/Blueprints/Interfaces/BPI_EquipmentSave.BPI_EquipmentSave_C")
      (bind (_found_ _data) (Class|BPIEquipmentSave|LoadEquipment(Message) (Game|GetGameInstance) (LocalVariables|GetLocalSaveName)))
      (if _found_
        (LocalVariables|SetLocalSaveData _data)
        (else
          (Utilities|PrintDebug (Utilities|String|Append "Equipment: Loading aborted, LoadEquipment function hasnt found any save data in game instance with save name " (LocalVariables|GetLocalSaveName)) "(R=0.968750,G=0.035319,B=0.035319,A=1.000000)" 6.0)
          (return false)))
      (else
        (Utilities|PrintDebug "Equipment: Loading aborted, game instance doesnt implement equipment save interface" "(R=0.968750,G=0.035319,B=0.035319,A=1.000000)" 6.0)
        (return false)))
    (else
      (bind _output_get_2 (LocalVariables|SetLocalSaveObject (CallFunction|GetEquipmentSaveObject)))
      (Utilities|IsValid _output_get_2
        (:Is%20Valid
          (bind (_found__2 _data_2) (Class|BPIEquipmentSave|LoadEquipment(Message) (LocalVariables|GetLocalSaveObject) (LocalVariables|GetLocalSaveName)))
          (if _found__2
            (LocalVariables|SetLocalSaveData _data_2)
            (else
              (Utilities|PrintDebug (Utilities|String|Append "Equipment: Loading aborted, LoadEquipment function hasnt found any save data in save object file with save name " (LocalVariables|GetLocalSaveName)) "(R=0.968750,G=0.035319,B=0.035319,A=1.000000)" 6.0)
              (return false))))
        (:Is%20Not%20Valid
          (Utilities|PrintDebug "Equipment: Loading aborted, GetEquipmentSaveObject has returned a not valid object reference" "(R=0.968750,G=0.035319,B=0.035319,A=1.000000)" 6.0)
          (return false)))))
  (Utilities|IsValid _returnvalue_2
    (:Is%20Valid
      (Variables|Default|SetPlayerInventoryReference _returnvalue_2)
      (bind _keys (Utilities|Map|Keys (Utilities|Struct|Breaks_EquipmentSaveData (LocalVariables|GetLocalSaveData))))
      (for _array_element _keys
        (bind _output_get_3 (LocalVariables|SetLocalEquipmentItem (.Value (Utilities|Map|Find (Utilities|Struct|Breaks_EquipmentSaveData (LocalVariables|GetLocalSaveData)) _array_element))))
        (if (Utilities|Name|NotEqual(Name) _output_get_3 "None")
          (bind _output_get_4 (LocalVariables|SetLocalItemData (CallFunction|GetItemDatabyRow (LocalVariables|GetLocalEquipmentItem))))
          (if (Utilities|IsValidClass (Utilities|Struct|Breaks_ItemData _output_get_4))
            (bind _returnvalue_3 (Game|SpawnActorfromClass (Utilities|Struct|Breaks_ItemData _output_get_4) (Math|Transform|MakeTransform "0, 0, 0" "0, 0, 0" "1,1,1") "Undefined" 0 (LocalVariables|GetLocalEquipmentItem) (LocalVariables|GetLocalItemData) (Variables|Default|GetPlayerInventoryReference) 0))
            (Default|AddSpawnedActor (Variables|Default|GetPlayerInventoryReference) (LocalVariables|GetLocalEquipmentItem) _returnvalue_3))
          (Managment|EquipItem (LocalVariables|GetLocalEquipmentItem) -1)))
      (Variables|Internal|SetHasLoadBeenSuccessful? true)
      (return true))
    (:Is%20Not%20Valid
      (Utilities|PrintDebug "Equipment Loading aborted, your player doesnt have the PlayerInventory component" "(R=0.994792,G=0.070239,B=0.000000,A=1.000000)" 5.0)
      (return false))))

(fn SetupEquipment
  (bind _enumvalue (|ForEache_EquipmentType)
    (:LoopBody
      (Utilities|Map|Add (Variables|General|GetEquipment) _enumvalue (LocalVariables|GetLocalNone)))
    (:then
      (return))))

(fn CreateEquipmentSaveData
  (return (Utilities|Struct|Makes_EquipmentSaveData (Variables|General|GetEquipment))))